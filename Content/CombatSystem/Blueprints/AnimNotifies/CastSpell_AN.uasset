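; CastSpell_AN is an animation notify that spawns a combat character's current spell when a cast animation reaches it.
; It casts the mesh owner to BP_CombatCharacter and spawns that character's CurrentSpell class at a configurable socket, facing the actor's forward vector, with the character as instigator.
; It then modifies a stat through StatsComponent by a fixed amount without regeneration and gives the spawned spell a short lifespan.
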(fn `Received_Notify`
  (params (MeshComp :type "SkeletalMeshComponent Object Reference") (Animation :type "AnimSequenceBase Object Reference") (EventReference :type "AnimNotifyEventReference Structure (by ref)"))
  (returns (ReturnValue :type Boolean))
  (bind _asbp_combat_character (cast `/Game/CombatSystem/Blueprints/BP_CombatCharacter` (`ActorComponent.GetOwner` MeshComp)))
  (bind _returnvalue (`|SpawnActorFromClass` (`/Game/CombatSystem/Blueprints/BP_CombatCharacter.CurrentSpell` _asbp_combat_character) (`KismetMathLibrary.MakeTransform` (`SceneComponent.GetSocketLocation` MeshComp (`self.InSocketName`)) (`KismetMathLibrary.MakeRotFromX` (`Actor.GetActorForwardVector` _asbp_combat_character))) "AlwaysSpawn" "OverrideRootScale" null _asbp_combat_character))
  (`/Game/CombatSystem/Blueprints/Components/BP_StatsComponent.ModifyCurrentStatValue` (`/Game/CombatSystem/Blueprints/BP_CombatCharacter.StatsComponent` _asbp_combat_character) "NewEnumerator5" 5.0 false)
  (`/Engine/EditorBlueprintResources/StandardMacros.IsValid` _returnvalue
    (:`Is Valid`
      (`Actor.SetLifeSpan` _returnvalue 0.5))
    (:`Is Not Valid`
      _))
  (return true))