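; BP_Consumable is a limited-use item actor, such as a health potion, that modifies a stat on its owning character.
; Its use count starts at the maximum, and PerformItemAction asks the owner to play the use montage as a gameplay-tagged action while uses remain.
; A separate ConsumeItem event decrements the count, sends the owner the potion amount update and applies the configured change through BP_StatsComponent.
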(event `self.ReceiveBeginPlay`
  ;[1 1 1] Begin Play
  (`parent.ReceiveBeginPlay`)
  (set `self.CurrentNumberOfUses` (`self.MaxNumberOfUses`)))

(event `self.PerformItemAction`
  ;[1 1 1] Use Item
  (if (> (`self.CurrentNumberOfUses`) 0)
    (message `/Game/CombatSystem/Blueprints/Interfaces/Combat_BPI.PerformCustomAction` (`self.GetOwner`) (struct :`TagName` "Character.Action.Use Item") (struct :`TagName` "Character.State.General Action State") (`self.UseItemMontgae`) 1.0 false)))

(event `ConsumeItem`
  ;[1 1 1] Consume Item
  (bind _result (`/Engine/EditorBlueprintResources/StandardMacros.DecrementInt` (`self.CurrentNumberOfUses`))
    (:`  `
      (message `/Game/CombatSystem/Blueprints/Interfaces/Combat_BPI.UpdateHealthPotionAmount` (`self.GetOwner`) _result)
      (`/Game/CombatSystem/Blueprints/Components/BP_StatsComponent.ModifyCurrentStatValue` (`self.GetComponentByClass` (`self.GetOwner`) "/Game/CombatSystem/Blueprints/Components/BP_StatsComponent.BP_StatsComponent_C") (`self.Stat`) (`self.ModificationValue`) (`self.ShouldRegenerate`)))))

(fn `UserConstructionScript`
  (`parent.UserConstructionScript`))