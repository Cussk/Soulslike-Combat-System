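; Base dual-wield weapon that adds an offhand mesh and right-foot hit detection to its parent weapon.
; On equip and combat toggle, the offhand mesh snaps to the owner's hand or attach socket.
; Collision components switch per body part, and offhand or foot hits apply point damage to actors that can receive it.
; DeactivateCollision calls ActivateCollision for the right foot, so that collision never turns off here.
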(event `self.ToggleWeaponCombat`
  (params (bEnableCombat :type Boolean))
  ;[1 1 1] Toggle Combat Event
  ;;[1 0 0] Attach offhand weapon to hand socket on combat enabled, and attach socket when disabled
  (`parent.ToggleWeaponCombat` bEnableCombat)
  (`self.AttachOffhandWeapon` (select `bool` bEnableCombat :`false` (`self.SecondWeaponAttachSocket`) :`true` (`self.SecondWeaponHandSocket`))))

(event `self.OffhandWeaponCollisionComponent.OnHit`
  (params (HitResult :type "HitResult Structure"))
  (bind (_bblockinghit _binitialoverlap _time _distance _location _impactpoint _normal _impactnormal _physmat _hitactor) (`GameplayStatics.BreakHitResult` HitResult))
  (bind _returnvalue (message `/Game/CombatSystem/Blueprints/Interfaces/Combat_BPI.CanReceiveDamage` _hitactor))
  (if _returnvalue
    (`GameplayStatics.ApplyPointDamage` _hitactor (`self.GetDamage`) (`self.GetActorForwardVector` (`self.GetOwner`)) HitResult (`self.GetInstigatorController`) self (`self.DamageTypeClass`))))

(event `self.RightFootCollisionComponent.OnHit`
  (params (HitResult :type "HitResult Structure"))
  (bind (_bblockinghit _binitialoverlap _time _distance _location _impactpoint _normal _impactnormal _physmat _hitactor) (`GameplayStatics.BreakHitResult` HitResult))
  (bind _returnvalue (message `/Game/CombatSystem/Blueprints/Interfaces/Combat_BPI.CanReceiveDamage` _hitactor))
  (if _returnvalue
    (`GameplayStatics.ApplyPointDamage` _hitactor (`self.GetDamage`) (`self.GetActorForwardVector` (`self.GetOwner`)) HitResult (`self.GetInstigatorController`) self (`self.DamageTypeClass`))))

(fn `ActivateCollision`
  (params (CollisionPart :type "/Game/CombatSystem/Blueprints/Enums/ECollisionPart Enum" :default "NewEnumerator0"))
  (switch `/Game/CombatSystem/Blueprints/Enums/ECollisionPart` CollisionPart
    (:`NewEnumerator0`
      (`/Game/CombatSystem/Blueprints/Components/BP_CollisionComponent.ActivateCollision` (`self.MainWeaponCollisionComponent`)))
    (:`NewEnumerator1`
      (`/Game/CombatSystem/Blueprints/Components/BP_CollisionComponent.ActivateCollision` (`self.OffhandWeaponCollisionComponent`)))
    (:`NewEnumerator2`
      (`/Game/CombatSystem/Blueprints/Components/BP_CollisionComponent.ActivateCollision` (`self.RightFootCollisionComponent`)))))

(fn `AttachOffhandWeapon`
  (params (Socket :type Name))
  (`SceneComponent.K2_AttachToComponent` (`self.OffhandItemStaticMesh`) (`Character.Mesh` (cast `Character` (`self.GetOwner`) :!pure true)) Socket "SnapToTarget" "SnapToTarget" "SnapToTarget" true))

(fn `DeactivateCollision`
  (params (collisionPart :type "/Game/CombatSystem/Blueprints/Enums/ECollisionPart Enum" :default "NewEnumerator0"))
  (switch `/Game/CombatSystem/Blueprints/Enums/ECollisionPart` collisionPart
    (:`NewEnumerator0`
      (`/Game/CombatSystem/Blueprints/Components/BP_CollisionComponent.DeactivateCollision` (`self.MainWeaponCollisionComponent`)))
    (:`NewEnumerator1`
      (`/Game/CombatSystem/Blueprints/Components/BP_CollisionComponent.DeactivateCollision` (`self.OffhandWeaponCollisionComponent`)))
    (:`NewEnumerator2`
      (`/Game/CombatSystem/Blueprints/Components/BP_CollisionComponent.ActivateCollision` (`self.RightFootCollisionComponent`)))))

(fn `OnEquipped`
  (`parent.OnEquipped`)
  (`/Game/CombatSystem/Blueprints/Components/BP_CollisionComponent.SetCollisionMeshComponent` (`self.OffhandWeaponCollisionComponent`) (`self.OffhandItemStaticMesh`))
  (`/Game/CombatSystem/Blueprints/Components/BP_CollisionComponent.SetCollisionMeshComponent` (`self.RightFootCollisionComponent`) (`Character.Mesh` (cast `Character` (`self.GetOwner`) :!pure true)))
  (`self.AttachOffhandWeapon` (select `bool` (`/Game/CombatSystem/Blueprints/Components/BP_CombatComponent.GetIsCombatEnabled` (`self.CombatComponent`)) :`false` (`self.SecondWeaponAttachSocket`) :`true` (`self.SecondWeaponHandSocket`)))
  (`/Game/CombatSystem/Blueprints/Components/BP_CollisionComponent.AddActorToIgnore` (`self.OffhandWeaponCollisionComponent`) (`self.GetOwner`))
  (`/Game/CombatSystem/Blueprints/Components/BP_CollisionComponent.AddActorToIgnore` (`self.RightFootCollisionComponent`) (`self.GetOwner`)))

(fn `UserConstructionScript`
  (`parent.UserConstructionScript`))