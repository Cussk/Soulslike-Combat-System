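; Base magic projectile for the combat system that deals point damage on overlap and explodes.
; When its sphere overlaps an actor that answers the CanReceiveDamage interface message positively, it applies GetDamage with its damage type, crediting the instigator's controller.
; It then plays impact sound and particles, stops and destroys itself, ignoring all other overlaps.
; The sphere's world location, rather than a direction vector, is passed as the hit direction.
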(event `self.Sphere.OnComponentBeginOverlap`
  (params (OverlappedComponent :type "PrimitiveComponent Object Reference") (OtherActor :type "Actor Object Reference") (OtherComp :type "PrimitiveComponent Object Reference") (OtherBodyIndex :type Integer) (bFromSweep :type Boolean) (SweepResult :type "HitResult Structure (by ref)"))
  (bind (_bblockinghit _binitialoverlap _time _distance _location _impactpoint _normal _impactnormal _physmat _hitactor) (`GameplayStatics.BreakHitResult` SweepResult))
  (bind _returnvalue (message `/Game/CombatSystem/Blueprints/Interfaces/Combat_BPI.CanReceiveDamage` _hitactor))
  (if _returnvalue
    (`GameplayStatics.ApplyPointDamage` _hitactor (`self.GetDamage`) (`SceneComponent.K2_GetComponentLocation` (`self.Sphere`)) SweepResult (`self.GetInstigatorController`) self (`self.DamageTypeClass`))
    (`self.OnHItExplode`)))

(fn `OnHItExplode`
  (`GameplayStatics.PlaySoundAtLocation` (`self.ImpactSound`) (`self.K2_GetActorLocation`) (struct) 1.0 1.0 0.0 null null null null)
  (`GameplayStatics.SpawnEmitterAtLocation` (`self.ParticleEmitter`) (`self.K2_GetActorLocation`) (`self.K2_GetActorRotation`))
  (`ActorComponent.Deactivate` (`self.ParticleSystem`))
  (`MovementComponent.StopMovementImmediately` (`self.ProjectileMovement`))
  (`self.K2_DestroyActor`))

(fn `UserConstructionScript`
  (`parent.UserConstructionScript`))