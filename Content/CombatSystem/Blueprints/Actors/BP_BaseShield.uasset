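; Base shield equippable for the combat system that registers itself as the owner's shield weapon when equipped and clears that slot when unequipped.
; On equip it binds to the combat-toggled event and attaches to the hand or holster socket based on combat state.
; Its collision component uses the item mesh and ignores the owner.
; A gameplay-tag switch supplies montages for attacks, blocking, dodging and entering or exiting combat.
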(fn `GetActionMontages`
  (params (CharacterAction :type "GameplayTag Structure"))
  (returns (Montages :type "Array of AnimMontage Object Reference"))
  (`|SwitchGameplayTag` CharacterAction
    (:`Character.Action.Attack.Light Attack`
      (return (`self.LightAttackMontages`)))
    (:`Character.Action.Attack.Heavy Attack`
      (return (`self.HeavyAttackMontages`)))
    (:`Character.Action.Attack.Charged Attack`
      (return (`self.ChargedAttackMontages`)))
    (:`Character.Action.Attack.Sprinting Attack`
      (return (`self.SprintingAttackMontages`)))
    (:`Character.Action.Attack.Falling Attack`
      (return (`self.FallingAttackMontages`)))
    (:`Character.Action.Block Attack`
      (return (`self.BlockAnimations`)))
    (:`Character.Action.Dodge`
      (return (`self.DodgeMontages`)))
    (:`Character.Action.Enter Combat`
      (return (`|MakeArray` (`self.EnterCombat`))))
    (:`Character.Action.Exit Combat`
      (return (`|MakeArray` (`self.ExitCombat`))))))

(fn `OnEquipped`
  (`self.SetIsEquipped` true)
  (`self.AttachActor` (`self.AttachSocketName`))
  ;[1 1 1] On Equip Sets Main Weapon
  (bind _output_get (set `self.CombatComponent` (`self.GetComponentByClass` (`self.GetOwner`) "/Game/CombatSystem/Blueprints/Components/BP_CombatComponent.BP_CombatComponent_C")))
  (add `/Game/CombatSystem/Blueprints/Components/BP_CombatComponent.OnCombatToggled` _output_get (`|CreateDelegate` :!event `ToggleWeaponCombat`))
  (set `self.OwnerStateManager` (`self.GetComponentByClass` (`self.GetOwner`) "/Game/CombatSystem/Blueprints/Components/BP_StateManagerComponent.BP_StateManagerComponent_C"))
  (`self.AttachActor` (select `bool` (`/Game/CombatSystem/Blueprints/Components/BP_CombatComponent.GetIsCombatEnabled` (`self.CombatComponent`)) :`false` (`self.AttachSocketName`) :`true` (`self.HandSocketName`)))
  (`/Game/CombatSystem/Blueprints/Components/BP_CombatComponent.SetShieldWeapon` (`self.CombatComponent`) self)
  ;[1 1 1] Sets collision mesh and ignore self from collisions
  (`/Game/CombatSystem/Blueprints/Components/BP_CollisionComponent.SetCollisionMeshComponent` (`self.MainWeaponCollisionComponent`) (`self.GetItemMesh`))
  (`/Game/CombatSystem/Blueprints/Components/BP_CollisionComponent.AddActorToIgnore` (`self.MainWeaponCollisionComponent`) (`self.GetOwner`)))

(fn `OnUnequipped`
  (`parent.OnUnequipped`)
  (`/Game/CombatSystem/Blueprints/Components/BP_CombatComponent.SetShieldWeapon` (`self.CombatComponent`) null))

(fn `UserConstructionScript`
  (`parent.UserConstructionScript`))