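; Combat stats component that holds an actor's base, max and current values per stat type, such as health, stamina and armor.
; Current values initialize from the base map, and modifications are clamped to the max, with each change broadcast.
; Only stamina regenerates, on a looping timer after a retriggerable delay.
; TakeDamage scales damage down by armor and sets the owner's state manager to Dead at zero health.
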(event `StartRegen`
  (params (StatType :type "/Game/CombatSystem/Blueprints/Enums/E_Stats Enum" :default "NewEnumerator0"))
  ;[1 1 1] Start Regen Event
  (switch `/Game/CombatSystem/Blueprints/Enums/E_Stats` StatType
    (:`NewEnumerator2`
      (`KismetSystemLibrary.K2_ClearTimer` null "RegenStamina")
      (`KismetSystemLibrary.RetriggerableDelay` 1.5)
      (`KismetSystemLibrary.K2_SetTimer` null "RegenStamina" 0.1 true))))

(fn `GetBaseStatsValue`
  (params (Stat :type "/Game/CombatSystem/Blueprints/Enums/E_Stats Enum" :default "NewEnumerator0"))
  (returns (BaseValue :type "Float (double-precision)"))
  (return (break `/Game/CombatSystem/Blueprints/Structs/F_BaseStats` (`BlueprintMapLibrary.Map_Find` (`self.BaseStats`) Stat))))

(fn `GetCurrentStatValue`
  (params (Stat :type "/Game/CombatSystem/Blueprints/Enums/E_Stats Enum" :default "NewEnumerator0"))
  (returns (Value :type "Float (double-precision)"))
  (return (`BlueprintMapLibrary.Map_Find` (`self.CurrentStats`) Stat)))

(fn `GetMaxStatsValue`
  (params (Stat :type "/Game/CombatSystem/Blueprints/Enums/E_Stats Enum" :default "NewEnumerator0"))
  (returns (MaxValue :type "Float (double-precision)"))
  (return (`.MaxValue_7_8A4FD7C34F2D6FEC7AD45C9FF89D4A7D` (break `/Game/CombatSystem/Blueprints/Structs/F_BaseStats` (`BlueprintMapLibrary.Map_Find` (`self.BaseStats`) Stat)))))

(fn `InitializeStats`
  (bind _keys (`BlueprintMapLibrary.Map_Keys` (`self.BaseStats`)))
  (for _array_element _keys
    (`self.SetCurrentStatValue` _array_element (break `/Game/CombatSystem/Blueprints/Structs/F_BaseStats` (`BlueprintMapLibrary.Map_Find` (`self.BaseStats`) _array_element)))))

(fn `ModifyCurrentStatValue`
  (params (Stat :type "/Game/CombatSystem/Blueprints/Enums/E_Stats Enum" :default "NewEnumerator0") (Value :type "Float (double-precision)") (bShouldRegenerate :type Boolean :default true))
  (locals (L_Value :type "Float (double-precision)"))
  ;[1 1 1] If value not zero, set current stat value to (current stat value + input stat value), value is clamped and updates Current Stat Value
  (if (!= Value 0.0)
    (bind _output_get (set `local.L_Value` (+ (`self.GetCurrentStatValue` (`local.Stat`)) (`local.Value`))))
    (bind _output_get_2 (set `local.L_Value` (`KismetMathLibrary.FClamp` _output_get 0.0 (`self.GetMaxStatsValue` (`local.Stat`)))))
    (`self.SetCurrentStatValue` (`local.Stat`) _output_get_2)
    ;[1 1 1] If should regnerate true start regen of stat
    (if (`local.bShouldRegenerate`)
      (`self.StartRegen` (`local.Stat`)))))

(fn `RegenStamina`
  (`self.SetCurrentStatValue` "NewEnumerator2" (`KismetMathLibrary.FClamp` (+ (`self.GetCurrentStatValue` "NewEnumerator2") (`self.StaminaRegenRate`)) 0.0 (`self.GetMaxStatsValue` "NewEnumerator2")))
  (if (>= (`self.GetCurrentStatValue` "NewEnumerator2") (`self.GetMaxStatsValue` "NewEnumerator2"))
    (`KismetSystemLibrary.K2_ClearTimer` null "RegenStamina")))

(fn `SetBaseStatValue`
  (params (Stat :type "/Game/CombatSystem/Blueprints/Enums/E_Stats Enum" :default "NewEnumerator0") (Value :type "Float (double-precision)"))
  ;[1 1 1] Set base stats update copy of value, add back into map to update original value
  (bind _structout (setmembers `/Game/CombatSystem/Blueprints/Structs/F_BaseStats` :`StructRef` (`BlueprintMapLibrary.Map_Find` (`self.BaseStats`) Stat) :`Base Value` Value))
  (`BlueprintMapLibrary.Map_Add` (`self.BaseStats`) (`local.Stat`) _structout))

(fn `SetCurrentStatValue`
  (params (Stat :type "/Game/CombatSystem/Blueprints/Enums/E_Stats Enum" :default "NewEnumerator0") (Value :type "Float (double-precision)"))
  (`BlueprintMapLibrary.Map_Add` (`self.CurrentStats`) Stat Value)
  (`self.OnCurrentStatValueUpdated` (`local.Stat`) (`local.Value`)))

(fn `SetMaxStatValue`
  (params (Stat :type "/Game/CombatSystem/Blueprints/Enums/E_Stats Enum" :default "NewEnumerator0") (Value :type "Float (double-precision)"))
  ;[1 1 1] Set max stats update copy of value, add back into map to update original value
  (bind _structout (setmembers `/Game/CombatSystem/Blueprints/Structs/F_BaseStats` :`StructRef` (`BlueprintMapLibrary.Map_Find` (`self.BaseStats`) Stat) :`Max Value` Value))
  (`BlueprintMapLibrary.Map_Add` (`self.BaseStats`) (`local.Stat`) _structout))

(fn `TakeDamage`
  (params (InDamage :type "Float (double-precision)"))
  (locals (L_Damage :type "Float (double-precision)"))
  (bind _returnvalue (* (`local.InDamage`) (/ (`local.InDamage`) (+ (`local.InDamage`) (`self.GetCurrentStatValue` "NewEnumerator3")))))
  (set `local.L_Damage` (`KismetMathLibrary.FClamp` _returnvalue 0.0 _returnvalue))
  (`self.ModifyCurrentStatValue` "NewEnumerator1" (* -1.0 (`local.L_Damage`)))
  (if (<= (`self.GetCurrentStatValue` "NewEnumerator1") 0.0)
    (`/Game/CombatSystem/Blueprints/Components/BP_StateManagerComponent.SetCurrentState` (`Actor.GetComponentByClass` (`self.GetOwner`) "/Game/CombatSystem/Blueprints/Components/BP_StateManagerComponent.BP_StateManagerComponent_C") (struct :`TagName` "Character.State.Dead"))))