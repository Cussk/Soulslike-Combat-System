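; Equipment component that manages a character's equipped items as spawned actors and triggers their actions by gameplay tag.
; InitializeEquipment unequips current items, then equips each class in StartingEquipment.
; EquipItem replaces any same-class item, spawning the new actor with the owning pawn as owner and instigator; UnequipItem destroys the actor without removing its array entry.
; Tag functions search EquippedItems for the first valid match to return or use.
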(fn `EquipItem`
  (params (InEquipment :type "/Game/CombatSystem/Blueprints/Actors/BP_BaseEquipable Class Reference"))
  (returns (bIsSuccessful :type Boolean))
  (bind _returnvalue (`self.GetOwner`))
  (bind _aspawn (cast `Pawn` _returnvalue :!pure true))
  (if (`KismetSystemLibrary.IsValidClass` InEquipment)
    (`|ExecutionSequence`
      (:`then_0`
        ;[1 1 1] If equipment already exists unequip
        (for _array_element (`self.EquippedItems`)
          (if (== (`GameplayStatics.GetObjectClass` _array_element) (`local.InEquipment`))
            (`self.UnequipItem` _array_element))))
      (:`then_1`
        ;[1 1 1] Equip New Equipment
        (bind _returnvalue_2 (`|SpawnActorFromClass` (`local.InEquipment`) (`Actor.GetTransform` _returnvalue) "Undefined" "OverrideRootScale" _aspawn _aspawn))
        (`/Game/CombatSystem/Blueprints/Actors/BP_BaseEquipable.OnEquipped` _returnvalue_2)
        (`KismetArrayLibrary.Array_AddUnique` (`self.EquippedItems`))
        (return true)))
    (else
      (return false))))

(fn `GetEquippedItemByTag`
  (params (ItemTag :type "GameplayTag Structure"))
  (returns (ReturnValue :type "/Game/CombatSystem/Blueprints/Actors/BP_BaseEquipable Object Reference"))
  (for _array_element (`self.EquippedItems`)
    (`/Engine/EditorBlueprintResources/StandardMacros.IsValid` _array_element
      (:`Is Valid`
        (bind _returnvalue (`/Game/CombatSystem/Blueprints/Actors/BP_BaseEquipable.HasMatchingGameplayTag` _array_element (`local.ItemTag`)))
        (if _returnvalue
          (return _array_element)))))
  (return null))

(fn `InitializeEquipment`
  (`|ExecutionSequence`
    (:`then_0`
      (for _array_element (`self.EquippedItems`)
        (`self.UnequipItem` _array_element)))
    (:`then_1`
      (for _array_element_2 (`self.StartingEquipment`)
        (if (`KismetSystemLibrary.IsValidClass` _array_element_2)
          (`self.EquipItem` _array_element_2))))))

(fn `PerformActionFromItem`
  (params (ItemTag :type "GameplayTag Structure"))
  ;[1 1 1] Lop through items character if matching gameplay tag use item
  (for _array_element (`self.EquippedItems`)
    (`/Engine/EditorBlueprintResources/StandardMacros.IsValid` _array_element
      (:`Is Valid`
        (bind _returnvalue (message `/Game/CombatSystem/Blueprints/Interfaces/GameplayTag_BPI.HasMatchingGameplayTag` _array_element (`local.ItemTag`)))
        (if _returnvalue
          (`/Game/CombatSystem/Blueprints/Actors/BP_BaseEquipable.PerformItemAction` _array_element)
          (return)))))
  (return))

(fn `UnequipItem`
  (params (EquipmentToUnequip :type "/Game/CombatSystem/Blueprints/Actors/BP_BaseEquipable Object Reference"))
  (`/Engine/EditorBlueprintResources/StandardMacros.IsValid` EquipmentToUnequip
    (:`Is Valid`
      (`/Game/CombatSystem/Blueprints/Actors/BP_BaseEquipable.OnUnequipped` EquipmentToUnequip)
      (`Actor.K2_DestroyActor` (`local.EquipmentToUnequip`)))))