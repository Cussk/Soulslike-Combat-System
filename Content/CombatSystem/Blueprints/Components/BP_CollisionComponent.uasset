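; Combat component that detects melee-style hits by tracing between two sockets on an assigned mesh while collision is active.
; While enabled, Tick runs a multi sphere trace for configured object types, skipping ignored actors.
; Each actor is recorded and reported once through OnHit per activation, since activating clears the already-hit list.
; Getters and setters expose the mesh, ignore list, last hit and collision state.
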(event `ActivateCollision`
  (`self.ClearHitActors`)
  (set `self.bIsCollisionEnabled` true))

(event `CollisonTrace`
  (bind _collisionmeshcomponent (`self.CollisionMeshComponent`))
  (bind _outhits (`KismetSystemLibrary.SphereTraceMultiForObjects` (`SceneComponent.GetSocketLocation` _collisionmeshcomponent (`self.StartSocketName`)) (`SceneComponent.GetSocketLocation` _collisionmeshcomponent (`self.EndSocketName`)) (`self.TraceRadius`) (`self.CollisionObjectTypes`) false (`self.ActorsToIgnore`) (`self.DrawDebugType`)))
  (for _array_element _outhits
    ;[1 1 1] Check if actor is in already hit array, if not in array, hit and add to array
    (bind _output_get (set `self.LastHit` _array_element))
    (bind (_bblockinghit _binitialoverlap _time _distance _location _impactpoint _normal _impactnormal _physmat _hitactor) (`GameplayStatics.BreakHitResult` _output_get))
    (if (not (`KismetArrayLibrary.Array_Contains` (`self.AlreadyHitActors`) _hitactor))
      (bind _output_get_2 (set `self.HitActor` _hitactor))
      (`KismetArrayLibrary.Array_Add` (`self.AlreadyHitActors`) _output_get_2)
      (`self.OnHit` (`self.LastHit`)))))

(event `DeactivateCollision`
  (set `self.bIsCollisionEnabled` false))

(event `ClearHitActors`
  (`KismetArrayLibrary.Array_Clear` (`self.AlreadyHitActors`)))

(event `self.ReceiveTick`
  (params (DeltaSeconds :type "Float (single-precision)"))
  (if (`self.bIsCollisionEnabled`)
    (`self.CollisonTrace`)))

(fn `AddActorToIgnore`
  (params (InActor :type "Actor Object Reference (by ref)"))
  (`KismetArrayLibrary.Array_AddUnique` (`self.ActorsToIgnore`) InActor))

(fn `GetActorsToIgnore`
  (returns (ReturnValue :type "Array of Actor Object Reference"))
  (return (`self.ActorsToIgnore`)))

(fn `GetAlreadyHitActors`
  (returns (ReturnValue :type "Array of Actor Object Reference"))
  (return (`self.AlreadyHitActors`)))

(fn `GetCollisionMeshComponent`
  (returns (ReturnValue :type "PrimitiveComponent Object Reference"))
  (return (`self.CollisionMeshComponent`)))

(fn `GetIsCollisionEnabled`
  (returns (ReturnValue :type Boolean))
  (return (`self.bIsCollisionEnabled`)))

(fn `GetLastHit`
  (returns (ReturnValue :type "HitResult Structure"))
  (return (`self.LastHit`)))

(fn `RemoveActorToIgnore`
  (params (InActor :type "Actor Object Reference (by ref)"))
  (`KismetArrayLibrary.Array_RemoveItem` (`self.ActorsToIgnore`) InActor))

(fn `SetCollisionMeshComponent`
  (params (MeshComponent :type "PrimitiveComponent Object Reference"))
  (set `self.CollisionMeshComponent` MeshComponent))