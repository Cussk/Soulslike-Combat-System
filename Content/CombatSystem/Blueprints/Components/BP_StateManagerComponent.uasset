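; BP_StateManagerComponent is a combat system component that tracks its owner's current state and current action as gameplay tags.
; Setting a different state or action fires the End dispatcher for the old tag, stores the new one, then fires the Begin dispatcher.
; Reset functions call the setters with a default tag, and query functions test the current tag against a tag container by exact match.
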(fn `GetCurrentAction`
  (returns (ReturnValue :type "GameplayTag Structure"))
  (return (`self.CurrentAction`)))

(fn `GetCurrentState`
  (returns (ReturnValue :type "GameplayTag Structure"))
  (return (`self.CurrentState`)))

(fn `IsCurrentActionEqualToAny`
  (params (ActionsToChcck :type "GameplayTagContainer Structure"))
  (returns (ReturnValue :type Boolean))
  ;[1 1 1] Check if current action is an existing tag, return bool
  (return (`BlueprintGameplayTagLibrary.HasTag` ActionsToChcck (`self.CurrentAction`) true)))

(fn `IsCurrentStateEqualToAny`
  (params (StatesToCheck :type "GameplayTagContainer Structure"))
  (returns (ReturnValue :type Boolean))
  ;[1 1 1] Check if current state is an existing tag, return bool
  (return (`BlueprintGameplayTagLibrary.HasTag` StatesToCheck (`self.CurrentState`) true)))

(fn `ResetAction`
  (`self.SetCurrentAction` (struct)))

(fn `ResetState`
  (`self.SetCurrentState` (struct)))

(fn `SetCurrentAction`
  (params (NewAction :type "GameplayTag Structure"))
  ;[1 1 1] If new action not equal to current action call end action, set current action to new action, call begin action with new current action
  (if (!= NewAction (`self.CurrentAction`))
    (`self.OnActionEnd` (`self.CurrentAction`))
    (bind _output_get (set `self.CurrentAction` (`local.NewAction`)))
    (`self.OnActionBegin` _output_get)))

(fn `SetCurrentState`
  (params (NewState :type "GameplayTag Structure"))
  ;[1 1 1] If new state not equal to current state call end state, set current state to new state, call begin state with new current state
  (if (!= NewState (`self.CurrentState`))
    (`self.OnStateEnd` (`self.CurrentState`))
    (bind _output_get (set `self.CurrentState` (`local.NewState`)))
    (`self.OnStateBegin` _output_get)))