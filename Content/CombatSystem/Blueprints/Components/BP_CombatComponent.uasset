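; Actor component that holds a character's combat state: the main weapon, whether combat is enabled, and attack progress.
; Setting a new main weapon unequips and destroys the existing one before storing the replacement.
; Toggling combat stores the flag and forwards it to the owning Character's AnimInstance through an interface message.
; A reset function clears the attack count, attacking flag and saved-attack flag.
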(fn `GetCombatEnabled`
  (returns (ReturnValue :type Boolean))
  (return (`self.bCombatEnabled`)))

(fn `GetMainWeapon`
  (returns (ReturnValue :type "/Game/CombatSystem/Blueprints/Actors/BP_BaseWeapon Object Reference"))
  (return (`self.MainWeapon`)))

(fn `ResetAttack`
  (set `self.AttackCount` 0)
  (set `self.bIsAttacking` false)
  (set `self.bAttackSaved` false))

(fn `SetCombatEnabled`
  (params (bCombatEnabled :type Boolean))
  ;[1 1 1] Set CombatEnabled and update AnimInstance interface
  (bind _output_get (set `self.bCombatEnabled` bCombatEnabled))
  (message `/Game/CombatSystem/Blueprints/Interfaces/AnimInstance_BPI.UpdateCombatEnabled` (`SkeletalMeshComponent.GetAnimInstance` (`Character.Mesh` (cast `Character` (`self.GetOwner`) :!pure true))) _output_get))

(fn `SetMainWeapon`
  (params (NewWeapon :type "/Game/CombatSystem/Blueprints/Actors/BP_BaseWeapon Object Reference"))
  (bind _mainweapon (`self.MainWeapon`))
  (`|ExecutionSequence`
    (:`then_0`
      ;[1 1 1] If weapon already exists, unequip and destroy
      (`/Engine/EditorBlueprintResources/StandardMacros.IsValid` _mainweapon
        (:`Is Valid`
          (`/Game/CombatSystem/Blueprints/Actors/BP_BaseEquipable.OnUnequipped` _mainweapon)
          (`Actor.K2_DestroyActor` (`self.MainWeapon`)))))
    (:`then_1`
      ;[1 1 1] Set new weapon as main weapon
      (set `self.MainWeapon` (`local.NewWeapon`)))))