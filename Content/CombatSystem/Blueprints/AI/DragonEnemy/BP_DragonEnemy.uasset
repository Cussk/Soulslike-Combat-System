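; Dragon boss enemy with a health bar shown while it has a target, weapon and claw hit damage, stun reactions and death handling.
; Pawn sensing sets the target; a looping timer picks melee or special attacks (the ranged branch is unreachable) and moves into range via AIMoveTo.
; Montage combos end in timeline-driven turns that re-arm the loop.
; The special attack only starts flying, with no landing or aerial attack.
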(event `SetBossHealthVisibility`
  (params (bIsVisible :type Boolean :default false))
  ;[1 1 1] Set Boss Health Visibility
  (bind _bosshealthui (`self.BossHealthUI`)
    (:`then`
      (`Widget.SetVisibility` _bosshealthui (select `bool` (and bIsVisible (not (`self.GetIsDead`))) :`false` "Hidden" :`true` "Visible" :!type "ESlateVisibility Enum")))
    (:`else`)))

(event `self.ReceiveBeginPlay`
  ;[1 0 0] Begin Play
  (`parent.ReceiveBeginPlay`)
  (`/Game/CombatSystem/Blueprints/Components/BP_CollisionComponent.SetCollisionMeshComponent` (`self.MainWeaponCollisionComponent`) (`self.Mesh`))
  (bind _returnvalue (`|CreateWidget` "/Game/CombatSystem/UI/WB_BossHealth.WB_BossHealth_C" (`GameplayStatics.GetPlayerController` 0)))
  (set `self.BossHealthUI` _returnvalue)
  (`UserWidget.AddToViewport` (`self.BossHealthUI`) 0)
  (`self.CombatStart`))

(event `self.OnTargetSet`
  (params (NewTarget :type "Actor Object Reference"))
  ;[1 1 1] Display Boss Health when enemy targets player
  (`parent.OnTargetSet` NewTarget)
  (`self.SetBossHealthVisibility` (`KismetSystemLibrary.IsValid` NewTarget)))

(event `HitEvent`
  (params (Hit :type "HitResult Structure (by ref)"))
  (bind (_bblockinghit _binitialoverlap _time _distance _location _impactpoint _normal _impactnormal _physmat _hitactor) (`GameplayStatics.BreakHitResult` Hit))
  ;[1 1 1] On Hit Event
  (bind _returnvalue (message `/Game/CombatSystem/Blueprints/Interfaces/Combat_BPI.CanReceiveDamage` _hitactor))
  (if _returnvalue
    (`GameplayStatics.ApplyPointDamage` _hitactor (`/Game/CombatSystem/Blueprints/Components/BP_StatsComponent.GetCurrentStatValue` (`self.StatsComponent`) "NewEnumerator4") (`self.GetActorForwardVector`) Hit (`self.GetController`) self (`self.Damage Type Class`))))

(event `self.MainWeaponCollisionComponent.OnHit`
  (params (HitResult :type "HitResult Structure"))
  ;[1 1 1] Hit Events
  (`self.HitEvent` HitResult))

(event `self.OffhandWeaponCollisionComponent.OnHit`
  (params (HitResult :type "HitResult Structure"))
  ;[1 1 1] Hit Events
  (`self.HitEvent` HitResult))

(event `/Game/CombatSystem/Blueprints/Interfaces/Targeting_BPI.OnTargeted`
  (params (bIsTargeted :type Boolean))
  ;[1 1 1] Targeting Event
  (`parent.OnTargeted` bIsTargeted))

(event `self.RightClawWeaponComponent.OnHit`
  (params (HitResult :type "HitResult Structure"))
  ;[1 1 1] Hit Events
  (`self.HitEvent` HitResult))

(event `SimulateWeaponPhysics`
  (bind _returnvalue (`self.GetWeaponMesh`))
  ;[1 1 1] Simulate Physics
  (`PrimitiveComponent.SetCollisionProfileName` _returnvalue "PhysicsActor" true)
  (`PrimitiveComponent.SetSimulatePhysics` _returnvalue false))

(event `self.PerformDeath`
  ;[1 1 1] Perform Death
  (if (not (`self.GetIsDead`))
    (`self.SetIsDead` true)
    (if (`KismetArrayLibrary.Array_IsNotEmpty` (`self.DeathAnimation`))
      (`self.PlayAnimMontage` (`KismetArrayLibrary.Array_Random` (`self.DeathAnimation`)))
      (else
        (`self.EnableRagdoll`)))
    (`self.ApplyHitReactionPhysicsVelocity` (`KismetMathLibrary.SelectFloat` 2000.0 -2000.0 (`self.bIsHitFront`)))
    (`PrimitiveComponent.SetCollisionResponseToChannel` (`self.CapsuleComponent`) "ECC_Pawn" "ECR_Overlap")
    (`KismetSystemLibrary.Delay` 4.0)
    (`self.K2_DestroyActor`)
    (`self.SimulateWeaponPhysics`)))

(event `self.CombatComponent.OnCombatToggled`
  (params (bIsCombatEnabled :type Boolean))
  ;[1 1 1] Attach Weapon to sockets
  (`SceneComponent.K2_AttachToComponent` (`self.WeaponMesh`) (`self.Mesh`) (select `bool` bIsCombatEnabled :`false` (`self.AttachSocketName`) :`true` (`self.WeaponHandSocketName`)) "KeepRelative" "KeepRelative" "KeepRelative" true))

(event `self.ReceiveTick`
  (params (DeltaSeconds :type "Float (single-precision)"))
  ;[1 1 1] Strafe Logic
  (`self.GeneralCheck`
    (:`Can`
      (bind _target (`self.Target`)
        (:`then`
          (bind _bisalive (message `/Game/CombatSystem/Blueprints/Interfaces/Combat_BPI.IsAlive` _target))
          (if _bisalive
            (if (`self.bEnableTick`)
              (switch `/Game/CombatSystem/Blueprints/AI/Enums/E_AIMovementDirections` (`self.AIMovementDirections`)
                (:`NewEnumerator0`
                  (set `self.StrafeVector` (0.0 0.0 0.0)))
                (:`NewEnumerator1`
                  (set `self.bEnableTick` false)))
              (bind _target_2 (`self.Target`)
                (:`then`
                  (bind (_returnvalue_roll _returnvalue_pitch _returnvalue_yaw) (`KismetMathLibrary.BreakRotator` (`KismetMathLibrary.FindLookAtRotation` (`self.K2_GetActorLocation`) (`self.K2_GetActorLocation` _target_2))))
                  (`self.K2_SetActorRotation` (`KismetMathLibrary.MakeRotator` 0.0 0.0 _returnvalue_yaw)))
                (:`else`)))
            (else
              (`AnimInstance.StopSlotAnimation` (`self.CastAnimInstance`) 0.25 "DefaultSlot"))))
        (:`else`)))))

(event `CustomEvent_1`
  (params (InDamageType :type "/Game/CombatSystem/Blueprints/Enums/E_DamageType Enum" :default "NewEnumerator0"))
  ;[1 0 0] Apply Hit Reaction
  (switch `/Game/CombatSystem/Blueprints/Enums/E_DamageType` "NewEnumerator0"
    (:`NewEnumerator0`
      (`self.PerformBaseHitReaction` :!label _label))
    (:`NewEnumerator1`
      (goto _label))
    (:`NewEnumerator2`
      (`self.PerformKnockdown`))
    (:`NewEnumerator4`
      (`self.PerformStun`)
      (`|ExecutionSequence`
        (:`then_0`
          (bind (_direction _alpha) (`Timeline|Knockback`) ; 0.5s
            (:`Update`
              (bind _target (`self.Target`)
                (:`then`
                  (`self.K2_SetActorLocation` (`KismetMathLibrary.VLerp` (`self.K2_GetActorLocation`) (0.0 0.0 0.0) _alpha)))
                (:`else`)))))
        (:`then_1`
          (`self.ResetStun`))))))

(event `CombatStart`
  ;[1 1 1] Combat Main Logic
  (`KismetSystemLibrary.K2_SetTimerDelegate` (delegate `CombatLogic`) 0.2 true)
  (set `self.CombatStartHandle` (struct)))

(event `CombatLogic`
  ;[1 1 1] Combat Main Logic
  (bind _target (`self.Target`)
    (:`then`
      (bind _bisalive (message `/Game/CombatSystem/Blueprints/Interfaces/Combat_BPI.IsAlive` _target))
      (if (and _bisalive (not (`self.GetIsDead`)) (`self.bAllowBehave`) (`self.bEnableTick`))
        (if (<= (`self.AttackCounts`) 0)
          (`KismetSystemLibrary.Delay` 1.0)
          (set `self.AttackCounts` (`KismetMathLibrary.RandomIntegerInRange` 2 3))
          (`self.NextAttack`)
          (`/Engine/EditorBlueprintResources/StandardMacros.IncrementInt` (`self.FlyCooldown`))
          (else
            (`/Engine/EditorBlueprintResources/StandardMacros.DoOnce` false :!label _label_2
              (:`Completed`
                (set `self.AIMovementDirections` "NewEnumerator1")
                (if (< (`self.FlyCooldown`) 2)
                  (set `self.FlyCooldown` 0)
                  (set `self.AIAttackType` "NewEnumerator2")
                  (set `self.AttackDistance` 99999.0)
                  (`self.MoveToTarget` :!label _label_3)
                  (elif (>= (`self.TargetLocation`) 1500.0)
                    (if true
                      (set `self.AIAttackType` "NewEnumerator0")
                      (set `self.AttackDistance` 1500.0)
                      (goto _label_3)
                      (else
                        (set `self.AIAttackType` "NewEnumerator1")
                        (set `self.AttackDistance` 5000.0)
                        (goto _label_3)))))))))))
    (:`else`)))

(event `NextAttack`
  ;[1 1 1] Combat Main Logic
  (goto _label_2 :!via `Reset`))

(event `MoveToTarget`
  ;[1 1 1] Move to proper distance
  (`/Engine/EditorBlueprintResources/StandardMacros.DoOnce` false :!label _label_4
    (:`Completed`
      (bind _target (`self.Target`)
        (:`then`
          (set `CharacterMovementComponent.MaxWalkSpeed` 1200.0 (`self.CharacterMovement`))
          (`|AIMoveTo` self (0.0 0.0 0.0) _target (`self.AttackDistance`)
            (:`then`
              (set `self.bIsDirectionalMove` false))
            (:`OnSuccess`
              (set `self.AIMovementDirections` "NewEnumerator0")
              (set `self.bIsDirectionalMove` true)
              (set `CharacterMovementComponent.MaxWalkSpeed` 600.0 (`self.CharacterMovement`))
              (`self.StartAttack`)
              (goto _label_4 :!via `Reset`))))
        (:`else`)))))

(event `StartAttack`
  ;[1 1 1] Attack Combo
  (`self.GeneralCheck`
    (:`Can`
      (switch `/Game/CombatSystem/Blueprints/AI/Enums/E_AIAttackType` (`self.AIAttackType`)
        (:`NewEnumerator0`
          (`self.BiteAttack`)
          (`self.GeneralCheck`
            (:`Can`
              (if (<= (`self.TargetLocation`) 1200.0)
                (`self.StompAttack`)
                (elif (`KismetMathLibrary.RandomBool`)
                  (`self.ClawAttack`)))
              (`self.EndAttackCombo`))))
        (:`NewEnumerator1`
          (if (`KismetMathLibrary.RandomBool`)
            (`self.ClawAttack`)
            (else
              (`self.SpitFireOnGround`)))
          (`self.EndAttackCombo`))
        (:`NewEnumerator2`
          (`self.StartToFly`))))))

(event `StartToFly`
  ;[1 1 1] Attack Combo
  (bind _output_get (set `self.bIsFlying` true))
  (message `/Game/CombatSystem/Blueprints/Interfaces/Combat_BPI.SetFly` (`self.CastAnimInstance`) _output_get)
  (`CharacterMovementComponent.SetMovementMode` (`self.CharacterMovement`) "MOVE_Flying" 0)
  (`self.QuickRotation`)
  (`Timeline|TakeOffCurve`
    (:`Update`
      (`self.GeneralCheck`))))

(event `QuickRotation`
  (bind (_returnvalue_roll _returnvalue_pitch _returnvalue_yaw) (`KismetMathLibrary.BreakRotator` (`self.K2_GetActorRotation`)))
  ;[1 1 1] Attack Combo
  ;;[1 1 1] Quick Rotate to player
  (bind (_direction _alpha) (`Timeline|ShortRotation` :!via `PlayFromStart` :!label _label_5)
    (:`Update`
      (bind _target (`self.Target`)
        (:`then`
          (bind (_returnvalue_roll_2 _returnvalue_pitch_2 _returnvalue_yaw_2) (`KismetMathLibrary.BreakRotator` (`KismetMathLibrary.FindLookAtRotation` (`self.K2_GetActorLocation`) (`self.K2_GetActorLocation` _target))))
          (bind (_returnvalue_roll_3 _returnvalue_pitch_3 _returnvalue_yaw_3) (`KismetMathLibrary.BreakRotator` (`KismetMathLibrary.RLerp` (`KismetMathLibrary.MakeRotator` 0.0 0.0 _returnvalue_yaw) (`KismetMathLibrary.MakeRotator` 0.0 0.0 _returnvalue_yaw_2) _alpha true)))
          (`self.K2_SetActorRotation` (`KismetMathLibrary.MakeRotator` 0.0 0.0 _returnvalue_yaw_3)))
        (:`else`
          (goto _label_5 :!via `Stop`))))))

(event `/Game/CombatSystem/Blueprints/Interfaces/Combat_BPI.ActivateCollision`
  (params (CollisionPart :type "/Game/CombatSystem/Blueprints/Enums/ECollisionPart Enum" :default "NewEnumerator0"))
  ;[1 1 1] Activate/Deactivate Collisions
  (switch `/Game/CombatSystem/Blueprints/Enums/ECollisionPart` CollisionPart
    (:`NewEnumerator0`
      (`/Game/CombatSystem/Blueprints/Components/BP_CollisionComponent.ActivateCollision` (`self.MainWeaponCollisionComponent`)))
    (:`NewEnumerator1`
      (`/Game/CombatSystem/Blueprints/Components/BP_CollisionComponent.ActivateCollision` (`self.OffhandWeaponCollisionComponent`)))
    (:`NewEnumerator3`
      (`/Game/CombatSystem/Blueprints/Components/BP_CollisionComponent.ActivateCollision` (`self.RightClawWeaponComponent`)))))

(event `EndAttackCombo`
  ;[1 1 1] Attack Combo
  ;;[1 1 1] End Attack Combo
  (bind _result (`/Engine/EditorBlueprintResources/StandardMacros.DecrementInt` (`self.AttackCounts`))
    (:`  `
      (set `self.AttackCounts` _result)
      (set `self.Damage Type Class` "/Game/CombatSystem/Blueprints/DamageTypes/BP_AttackDamageType.BP_AttackDamageType_C")
      (`self.RotateToPlayer`))))

(event `/Game/CombatSystem/Blueprints/Interfaces/Combat_BPI.DeactivateCollision`
  (params (CollisionPart :type "/Game/CombatSystem/Blueprints/Enums/ECollisionPart Enum" :default "NewEnumerator0"))
  ;[1 1 1] Activate/Deactivate Collisions
  (switch `/Game/CombatSystem/Blueprints/Enums/ECollisionPart` CollisionPart
    (:`NewEnumerator0`
      (`/Game/CombatSystem/Blueprints/Components/BP_CollisionComponent.DeactivateCollision` (`self.MainWeaponCollisionComponent`)))
    (:`NewEnumerator1`
      (`/Game/CombatSystem/Blueprints/Components/BP_CollisionComponent.DeactivateCollision` (`self.OffhandWeaponCollisionComponent`)))
    (:`NewEnumerator3`
      (`/Game/CombatSystem/Blueprints/Components/BP_CollisionComponent.DeactivateCollision` (`self.RightClawWeaponComponent`)))))

(event `RotateToPlayer`
  (bind (_returnvalue_roll _returnvalue_pitch _returnvalue_yaw) (`KismetMathLibrary.BreakRotator` (`self.K2_GetActorRotation`)))
  ;[1 1 1] Rotate to player if relative angle is over 30
  (`self.GeneralCheck`
    (:`Can`
      (`self.Target`
        (:`then`
          (bind (_rotationtime _bneedtorotate) (`self.TurnInPlace`))
          (if _bneedtorotate
            (`TimelineComponent.SetPlayRate` (`self.RotateCurve`) (/ 1.0 (select `bool` (`KismetMathLibrary.NearlyEqual_FloatFloat` _rotationtime) :`false` _rotationtime :`true` 1.0)))
            (bind (_direction _alpha) (`Timeline|RotateCurve` :!via `PlayFromStart` :!label _label_6)
              (:`Update`
                (bind _target (`self.Target`)
                  (:`then`
                    (bind (_returnvalue_roll_2 _returnvalue_pitch_2 _returnvalue_yaw_2) (`KismetMathLibrary.BreakRotator` (`KismetMathLibrary.FindLookAtRotation` (`self.K2_GetActorLocation`) (`self.K2_GetActorLocation` _target))))
                    (bind (_returnvalue_roll_3 _returnvalue_pitch_3 _returnvalue_yaw_3) (`KismetMathLibrary.BreakRotator` (`KismetMathLibrary.RLerp` (`KismetMathLibrary.MakeRotator` 0.0 0.0 _returnvalue_yaw) (`KismetMathLibrary.MakeRotator` 0.0 0.0 _returnvalue_yaw_2) _alpha true)))
                    (`self.K2_SetActorRotation` (`KismetMathLibrary.MakeRotator` 0.0 0.0 _returnvalue_yaw_3)))
                  (:`else`
                    (goto _label_6 :!via `Stop`))))
              (:`Finished`
                (`self.GeneralCheck` :!label _label_7
                  (:`Can`
                    (set `self.bEnableTick` true)
                    (`self.NextAttack`)))))
            (else
              (goto _label_7))))
        (:`else`)))))

(event `FireStart`
  ;[1 1 1] Fire Particle Activate/Deactivate
  (`ActorComponent.Activate` (`self.ParticleSystem`) false))

(event `FireEnd`
  ;[1 1 1] Fire Particle Activate/Deactivate
  (`ActorComponent.Deactivate` (`self.ParticleSystem`)))

(event `self.PawnSensing.OnSeePawn`
  (params (Pawn :type "Pawn Object Reference"))
  ;[1 1 1] On See Pawn
  (set `self.Target` Pawn)
  (`/Engine/EditorBlueprintResources/StandardMacros.DoOnce` false
    (:`Completed`
      (set `self.bEnableTick` false)
      (`KismetSystemLibrary.Delay` 1.0)
      (`self.RotateToPlayer`)
      (set `self.FlyCooldown` 0))))

(fn `PerformStun`
  (returns (bIsSuccessful :type Boolean))
  (set `self.bEnableTick` false)
  (set `self.bAllowBehave` false)
  (bind _bissuccessful (`parent.PerformStun`))
  (return _bissuccessful))

(fn `TurnInPlace`
  (returns (RotationTime :type "Float (double-precision)") (bNeedToRotate :type Boolean))
  (locals (`L_RelativeRotation]` :type "Float (double-precision)") (L_RotationTime :type "Float (single-precision)" :default 0.0))
  (bind (_returnvalue_roll _returnvalue_pitch _returnvalue_yaw) (`KismetMathLibrary.BreakRotator` (`self.K2_GetActorRotation`)))
  (bind _l_relativerotation_ (`local.L_RelativeRotation]`))
  (bind _l_relativerotation__2 (`local.L_RelativeRotation]`))
  (bind _l_relativerotation__3 (`local.L_RelativeRotation]`))
  (bind _l_relativerotation__4 (`local.L_RelativeRotation]`))
  (bind _l_relativerotation__5 (`local.L_RelativeRotation]`))
  (bind _l_relativerotation__6 (`local.L_RelativeRotation]`))
  (bind _target (`self.Target`)
    (:`then`
      (bind (_returnvalue_roll_2 _returnvalue_pitch_2 _returnvalue_yaw_2) (`KismetMathLibrary.BreakRotator` (`KismetMathLibrary.FindLookAtRotation` (`self.K2_GetActorLocation`) (`self.K2_GetActorLocation` _target))))
      (set `local.L_RelativeRotation]` (- _returnvalue_yaw_2 _returnvalue_yaw))
      (if (or (and (> _l_relativerotation_ 0.0) (<= _l_relativerotation_ 90.0)) (and (< _l_relativerotation__2 -360.0) (>= _l_relativerotation__2 -270.0)))
        (`KismetSystemLibrary.PrintString` "Player is right forward of enemy")
        (bind _returnvalue (`self.PlayAnimMontage` "/Game/Assets/QuadrapedCreatures/MountainDragon/Animations/ANIM_MOUNTAIN_DRAGON_turn90Right_Montage.ANIM_MOUNTAIN_DRAGON_turn90Right_Montage"))
        (set `local.L_RotationTime` _returnvalue)
        (elif (or (and (> _l_relativerotation__3 90.0) (<= _l_relativerotation__3 180.0)) (and (< _l_relativerotation__4 -270.0) (>= _l_relativerotation__4 -180.0)))
          (`KismetSystemLibrary.PrintString` "Player right backward")
          (bind _returnvalue_2 (`self.PlayAnimMontage` "/Game/Assets/QuadrapedCreatures/MountainDragon/Animations/ANIM_MOUNTAIN_DRAGON_turn90Right_Montage.ANIM_MOUNTAIN_DRAGON_turn90Right_Montage"))
          (set `local.L_RotationTime` _returnvalue_2)
          (elif (or (and (> _l_relativerotation__5 180.0) (<= _l_relativerotation__5 270.0)) (and (< _l_relativerotation__6 -180.0) (>= _l_relativerotation__6 -90.0)))
            (`KismetSystemLibrary.PrintString` "Player left backward")
            (bind _returnvalue_3 (`self.PlayAnimMontage` "/Game/Assets/QuadrapedCreatures/MountainDragon/Animations/ANIM_MOUNTAIN_DRAGON_turn90Left_Montage.ANIM_MOUNTAIN_DRAGON_turn90Left_Montage"))
            (set `local.L_RotationTime` _returnvalue_3)
            (else
              (`KismetSystemLibrary.PrintString` "Player left forward")
              (bind _returnvalue_4 (`self.PlayAnimMontage` "/Game/Assets/QuadrapedCreatures/MountainDragon/Animations/ANIM_MOUNTAIN_DRAGON_turn90Left_Montage.ANIM_MOUNTAIN_DRAGON_turn90Left_Montage"))
              (set `local.L_RotationTime` _returnvalue_4)))))
      (return (`local.L_RotationTime`) true))
    (:`else`)))

(fn `UserConstructionScript`
  (`parent.UserConstructionScript`)
  (`SceneComponent.K2_SetRelativeLocation` (`self.Mesh`) (0.0 0.0 0.0) false false)
  (`SceneComponent.K2_AddRelativeLocation` (`self.Mesh`) (`KismetMathLibrary.MakeVector` 0.0 0.0 (- 0.0 (`CapsuleComponent.GetScaledCapsuleHalfHeight` (`self.CapsuleComponent`)))) false false))