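; BP_Fireball is an explosive fireball attack for the dragon enemy, with a six-second lifespan.
; Sphere overlap stops its particles, plays explosion effects and sound, and checks the hit actor through CanReceiveDamageMessage.
; Damageable actors take point damage credited to the Dragon, and only then is the fireball destroyed on overlap.
; A separate EndOfFirball event repeats the explosion without damage and destroys it after a short delay.
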(event `self.ReceiveBeginPlay`
  (`self.SetLifeSpan` 6.0))

(event `self.Sphere.OnComponentBeginOverlap`
  (params (OverlappedComponent :type "PrimitiveComponent Object Reference") (OtherActor :type "Actor Object Reference") (OtherComp :type "PrimitiveComponent Object Reference") (OtherBodyIndex :type Integer) (bFromSweep :type Boolean) (SweepResult :type "HitResult Structure (by ref)"))
  (bind (_bblockinghit _binitialoverlap _time _distance _location _impactpoint _normal _impactnormal _physmat _hitactor) (`GameplayStatics.BreakHitResult` SweepResult))
  (`ActorComponent.Deactivate` (`self.ParticleSystem`))
  (`GameplayStatics.SpawnEmitterAtLocation` "/Game/Assets/Realistic_Starter_VFX_Pack_Vol2/Particles/Explosion/P_Explosion_Big_A.P_Explosion_Big_A" (`self.K2_GetActorLocation`))
  (`GameplayStatics.PlaySoundAtLocation` "/Game/CombatSystem/CourseFiles/SoundFX/Ability_MeteorImpact_Cue.Ability_MeteorImpact_Cue" (`self.K2_GetActorLocation`) (struct) 1.0 1.0 0.0 null null null null)
  (bind _returnvalue (message `/Game/CombatSystem/Blueprints/Interfaces/Combat_BPI.CanReceiveDamage` _hitactor))
  (if _returnvalue
    (`GameplayStatics.ApplyPointDamage` _hitactor (`self.Base Damage`) (`SceneComponent.K2_GetComponentLocation` (`self.Sphere`)) SweepResult (`self.GetInstigatorController`) (`self.Dragon`) (`self.DamageTypeClass`))
    (`self.K2_DestroyActor`)))

(event `EndOfFirball`
  (`GameplayStatics.SpawnEmitterAtLocation` "/Game/Assets/Realistic_Starter_VFX_Pack_Vol2/Particles/Explosion/P_Explosion_Big_A.P_Explosion_Big_A" (`self.K2_GetActorLocation`))
  (`GameplayStatics.PlaySoundAtLocation` "/Game/CombatSystem/CourseFiles/SoundFX/Ability_MeteorImpact_Cue.Ability_MeteorImpact_Cue" (`self.K2_GetActorLocation`) (struct) 1.0 1.0 0.0 null null null null)
  (`KismetSystemLibrary.Delay` 0.1)
  (`self.K2_DestroyActor`))

(fn `UserConstructionScript`)