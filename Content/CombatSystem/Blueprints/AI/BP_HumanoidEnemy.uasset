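; BP_HumanoidEnemy is a humanoid enemy AI character in the combat system, with a health bar and weapon-based melee damage.
; On BeginPlay it creates a WB_HealthBar widget bound to its own StatsComponent, shown or hidden as it is targeted or untargeted.
; Hits from the main weapon collision component apply point damage, scaled from a stat, to actors that can receive damage, using the attack damage type.
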(event `self.ReceiveBeginPlay`
  (`parent.ReceiveBeginPlay`)
  (bind _returnvalue (`|CreateWidget` "/Game/CombatSystem/UI/WB_HealthBar.WB_HealthBar_C" (`GameplayStatics.GetPlayerController` 0) (`self.StatsComponent`) false))
  (`WidgetComponent.SetWidget` (`self.HealthBar`) _returnvalue))

(event `/Game/CombatSystem/Blueprints/Interfaces/Targeting_BPI.OnTargeted`
  (params (bIsTargeted :type Boolean))
  (`parent.OnTargeted` bIsTargeted)
  (`SceneComponent.SetVisibility` (`self.HealthBar`) bIsTargeted false))

(event `self.MainWeaponCollisionComponent_0.OnHit`
  (params (HitResult :type "HitResult Structure"))
  (bind (_bblockinghit _binitialoverlap _time _distance _location _impactpoint _normal _impactnormal _physmat _hitactor) (`GameplayStatics.BreakHitResult` HitResult))
  (bind _returnvalue (message `/Game/CombatSystem/Blueprints/Interfaces/Combat_BPI.CanReceiveDamage` _hitactor))
  (if _returnvalue
    (`GameplayStatics.ApplyPointDamage` _hitactor (`/Game/CombatSystem/Blueprints/Components/BP_StatsComponent.GetCurrentStatValue` (`self.StatsComponent`) "NewEnumerator4") (`self.GetActorForwardVector` (`self.GetOwner`)) HitResult (`self.GetInstigatorController`) self "/Game/CombatSystem/Blueprints/DamageTypes/BP_AttackDamageType.BP_AttackDamageType_C")))

(fn `UserConstructionScript`
  (`parent.UserConstructionScript`))