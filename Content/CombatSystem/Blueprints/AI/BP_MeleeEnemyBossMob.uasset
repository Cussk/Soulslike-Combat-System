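; Melee boss enemy Blueprint that targets the player on spawn and alternates attack runs with strafing.
; A looping timer picks close combos or timeline-driven leap attacks by distance, then recharges the attack count while tick-driven strafing circles or backs off, using box traces on collision.
; Attacks swap damage types for knockdown or stun, and turn-in-place timelines re-aim between combos.
; It also handles its own hit reactions, weapon socketing, targeted health bar and death.
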(event `self.MainWeaponCollisionComponent.OnHit`
  (params (HitResult :type "HitResult Structure"))
  (bind (_bblockinghit _binitialoverlap _time _distance _location _impactpoint _normal _impactnormal _physmat _hitactor) (`GameplayStatics.BreakHitResult` HitResult))
  ;[1 1 1] On Hit Event
  (bind _returnvalue (message `/Game/CombatSystem/Blueprints/Interfaces/Combat_BPI.CanReceiveDamage` _hitactor))
  (if _returnvalue
    (`GameplayStatics.ApplyPointDamage` _hitactor (`/Game/CombatSystem/Blueprints/Components/BP_StatsComponent.GetCurrentStatValue` (`self.StatsComponent`) "NewEnumerator4") (`self.GetActorForwardVector`) HitResult (`self.GetController`) self (`self.Damage Type Class`))))

(event `/Game/CombatSystem/Blueprints/Interfaces/Targeting_BPI.OnTargeted`
  (params (bIsTargeted :type Boolean))
  ;[1 1 1] Targeting Event
  (`parent.OnTargeted` bIsTargeted)
  (`SceneComponent.SetVisibility` (`self.HealthBar`) bIsTargeted false))

(event `self.ReceiveBeginPlay`
  ;[1 0 0] Begin Play
  (`parent.ReceiveBeginPlay`)
  (`|ExecutionSequence`
    (:`then_0`
      (`/Game/CombatSystem/Blueprints/Components/BP_CollisionComponent.SetCollisionMeshComponent` (`self.MainWeaponCollisionComponent`) (`self.WeaponMesh`))
      (bind _returnvalue (`|CreateWidget` "/Game/CombatSystem/UI/WB_HealthBar.WB_HealthBar_C" (`GameplayStatics.GetPlayerController` 0) (`self.StatsComponent`)))
      (`WidgetComponent.SetWidget` (`self.HealthBar`) _returnvalue)
      (`self.CombatStart`))
    (:`then_1`
      ;[1 1 1] On See Pawn
      (`/Engine/EditorBlueprintResources/StandardMacros.DoOnce` false
        (:`Completed`
          (set `self.Target` (`GameplayStatics.GetPlayerCharacter` 0))
          (set `self.bEnableTick` false)
          (`/Game/CombatSystem/Blueprints/Interfaces/Combat_BPI.PerformAction` (struct :`TagName` "Character.Action.Enter Combat"))
          (message `/Game/CombatSystem/Blueprints/Interfaces/AnimInstance_BPI.UpdateCombatType` (`self.CastAnimInstance`) "NewEnumerator1")
          (`KismetSystemLibrary.Delay` 1.0)
          (`self.RotateToPlayer`))))))

(event `SimulateWeaponPhysics`
  (bind _returnvalue (`self.GetWeaponMesh`))
  ;[1 1 1] Simulate Physics
  (`PrimitiveComponent.SetCollisionProfileName` _returnvalue "PhysicsActor" true)
  (`PrimitiveComponent.SetSimulatePhysics` _returnvalue false))

(event `self.PerformDeath`
  ;[1 1 1] Perform Death
  (if (not (`self.GetIsDead`))
    (`self.SetIsDead` true)
    (if (`KismetArrayLibrary.Array_IsNotEmpty` (`self.DeathAnimation`))
      (`self.PlayAnimMontage` (`KismetArrayLibrary.Array_Random` (`self.DeathAnimation`)))
      (else
        (`self.EnableRagdoll`)))
    (`self.ApplyHitReactionPhysicsVelocity` (`KismetMathLibrary.SelectFloat` 2000.0 -2000.0 (`self.bIsHitFront`)))
    (`PrimitiveComponent.SetCollisionResponseToChannel` (`self.CapsuleComponent`) "ECC_Pawn" "ECR_Overlap")
    (`KismetSystemLibrary.Delay` 4.0)
    (`self.K2_DestroyActor`)
    (`self.SimulateWeaponPhysics`)))

(event `self.CombatComponent.OnCombatToggled`
  (params (bIsCombatEnabled :type Boolean))
  ;[1 1 1] Attach Weapon to sockets
  (`SceneComponent.K2_AttachToComponent` (`self.WeaponMesh`) (`self.Mesh`) (select `bool` bIsCombatEnabled :`false` (`self.AttachSocketName`) :`true` (`self.WeaponHandSocketName`)) "KeepRelative" "KeepRelative" "KeepRelative" true))

(event `self.ReceiveTick`
  (params (DeltaSeconds :type "Float (single-precision)"))
  (bind (_returnvalue_roll _returnvalue_pitch _returnvalue_yaw) (`KismetMathLibrary.BreakRotator` (`KismetMathLibrary.NormalizedDeltaRotator` (`KismetMathLibrary.Conv_VectorToRotator` (`self.StrafeVector`)) (`self.GetControlRotation`))))
  ;[1 1 1] Strafe Logic
  (`self.GeneralCheck`
    (:`Can`
      (bind _target (`self.Target`)
        (:`then`
          (bind _bisalive (message `/Game/CombatSystem/Blueprints/Interfaces/Combat_BPI.IsAlive` _target))
          (if _bisalive
            (if (`self.bEnableTick`)
              (switch `/Game/CombatSystem/Blueprints/AI/Enums/E_AIMovementDirections` (`self.AIMovementDirections`)
                (:`NewEnumerator0`
                  (set `self.StrafeVector` (0.0 0.0 0.0)))
                (:`NewEnumerator1`
                  (set `self.bEnableTick` false))
                (:`NewEnumerator2`
                  (set `self.StrafeVector` (* (`self.GetActorForwardVector`) (`self.MinusOne`))))
                (:`NewEnumerator3`
                  (set `self.StrafeVector` (* (`self.GetActorRightVector`) (`self.MinusOne`))))
                (:`NewEnumerator4`
                  (set `self.StrafeVector` (`self.GetActorRightVector`))))
              (`self.AddMovementInput` (`self.StrafeVector`))
              (message `/Game/CombatSystem/Blueprints/Interfaces/Combat_BPI.DirectionValue` (`self.CastAnimInstance`) (select `bool` (`self.bIsDirectionalMove`) :`true` _returnvalue_yaw :!type "Float (double-precision)"))
              (bind _target_2 (`self.Target`)
                (:`then`
                  (bind (_returnvalue_roll_2 _returnvalue_pitch_2 _returnvalue_yaw_2) (`KismetMathLibrary.BreakRotator` (`KismetMathLibrary.FindLookAtRotation` (`self.K2_GetActorLocation`) (`self.K2_GetActorLocation` _target_2))))
                  (`self.K2_SetActorRotation` (`KismetMathLibrary.MakeRotator` 0.0 0.0 _returnvalue_yaw_2)))
                (:`else`)))
            (else
              (`AnimInstance.StopSlotAnimation` (`self.CastAnimInstance`) 0.25 "DefaultSlot"))))
        (:`else`)))))

(event `CustomEvent_1`
  (params (InDamageType :type "/Game/CombatSystem/Blueprints/Enums/E_DamageType Enum" :default "NewEnumerator0"))
  ;[1 0 0] Apply Hit Reaction
  (switch `/Game/CombatSystem/Blueprints/Enums/E_DamageType` "NewEnumerator0"
    (:`NewEnumerator0`
      (`self.PerformBaseHitReaction` :!label _label))
    (:`NewEnumerator1`
      (goto _label))
    (:`NewEnumerator2`
      (`self.PerformKnockdown`))
    (:`NewEnumerator4`
      (`self.PerformStun`)
      (`|ExecutionSequence`
        (:`then_0`
          (bind (_direction _alpha) (`Timeline|Knockback`) ; 0.5s
            (:`Update`
              (bind _target (`self.Target`)
                (:`then`
                  (`self.K2_SetActorLocation` (`KismetMathLibrary.VLerp` (`self.K2_GetActorLocation`) (0.0 0.0 0.0) _alpha)))
                (:`else`)))))
        (:`then_1`
          (`self.ResetStun`))))))

(event `CombatStart`
  ;[1 1 1] Combat Main Logic
  (`KismetSystemLibrary.K2_SetTimerDelegate` (delegate `CombatLogic`) 0.2 true)
  (set `self.CombatStartHandle` (struct)))

(event `CombatLogic`
  ;[1 1 1] Combat Main Logic
  (bind _target (`self.Target`)
    (:`then`
      (bind _bisalive (message `/Game/CombatSystem/Blueprints/Interfaces/Combat_BPI.IsAlive` _target))
      (if (and _bisalive (not (`self.GetIsDead`)) (`self.bAllowBehave`) (`self.bEnableTick`))
        (if (<= (`self.AttackCounts`) 0)
          ;;[1 1 1] 1. Recharge Attack Counts
          ;; 2. Strafe Logic
          (`|ExecutionSequence`
            (:`then_0`
              ;;[1 1 1] Strafing State for 5 seconds then begin next attack
              (`KismetSystemLibrary.Delay` 5.0)
              (set `self.AttackCounts` (`KismetMathLibrary.RandomIntegerInRange` 2 3))
              (`self.NextAttack`))
            (:`then_1`
              (`/Engine/EditorBlueprintResources/StandardMacros.DoOnce` false :!label _label_2
                (:`Completed`
                  (set `self.bIsStrafing` true :!label _label_3)
                  (if (and (<= (`self.TargetLocation`) 200.0) (not (`self.IsColliding`)))
                    (`KismetSystemLibrary.PrintString` "AI Go Backward")
                    (set `self.AIMovementDirections` "NewEnumerator2")
                    (else
                      (`KismetSystemLibrary.PrintString` "AI Go Left or Right")
                      (if (`KismetMathLibrary.RandomBool`)
                        (set `self.AIMovementDirections` "NewEnumerator3")
                        (else
                          (set `self.AIMovementDirections` "NewEnumerator4")))))))))
          (else
            (`/Engine/EditorBlueprintResources/StandardMacros.DoOnce` false :!label _label_4
              (:`Completed`
                (`|ExecutionSequence`
                  (:`then_0`
                    (set `self.bIsStrafing` false)
                    (set `self.AIMovementDirections` "NewEnumerator1")
                    (if (<= (`self.TargetLocation`) 800.0)
                      (set `self.AIAttackType` "NewEnumerator0")
                      (set `self.AttackDistance` 150.0)
                      (else
                        (set `self.AIAttackType` "NewEnumerator1")
                        (set `self.AttackDistance` 2000.0)))
                    (`self.MoveToTarget`))
                  (:`then_1`
                    (goto _label_2 :!via `Reset`)))))))))
    (:`else`)))

(event `NextAttack`
  ;[1 1 1] Combat Main Logic
  (goto _label_4 :!via `Reset`))

(event `StartStrafe`
  ;[1 1 1] Combat Main Logic
  (goto _label_3))

(event `MoveToTarget`
  ;[1 1 1] Mov to proper distance
  (`/Engine/EditorBlueprintResources/StandardMacros.DoOnce` false :!label _label_5
    (:`Completed`
      ;;[1 1 1] Disable Strafe
      (set `self.StrafeVector` (0.0 0.0 0.0))
      (bind _target (`self.Target`)
        (:`then`
          (set `CharacterMovementComponent.MaxWalkSpeed` 700.0 (`self.CharacterMovement`))
          (`|AIMoveTo` self (0.0 0.0 0.0) _target (`self.AttackDistance`)
            (:`then`
              (set `self.bIsDirectionalMove` false))
            (:`OnSuccess`
              (set `self.AIMovementDirections` "NewEnumerator0")
              (set `self.bIsDirectionalMove` true)
              (set `CharacterMovementComponent.MaxWalkSpeed` 400.0 (`self.CharacterMovement`))
              (`self.StartAttack`)
              (goto _label_5 :!via `Reset`))))
        (:`else`)))))

(event `StartAttack`
  (bind _target (`self.Target`))
  ;[1 1 1] Attack Combo
  (`self.GeneralCheck`
    (:`Can`
      (switch `/Game/CombatSystem/Blueprints/AI/Enums/E_AIAttackType` (`self.AIAttackType`)
        (:`NewEnumerator0`
          (`self.NormalAttack`)
          (`self.GeneralCheck` :!label _label_6
            (:`Can`
              (if (<= (`self.TargetLocation`) 220.0)
                (`self.StunAttack`)
                (`self.EndAttackCombo`)
                (else
                  (`self.EndAttackCombo`))))))
        (:`NewEnumerator1`
          (set `self.Damage Type Class` "/Game/CombatSystem/Blueprints/DamageTypes/BP_KnockdownAttackDamageType.BP_KnockdownAttackDamageType_C")
          (bind _returnvalue (`self.PlayAnimMontage` (`KismetArrayLibrary.Array_Random` (`self.LongRangeAttackMontages`))))
          (`|ExecutionSequence`
            (:`then_0`
              (`KismetSystemLibrary.Delay` (+ _returnvalue 0.2))
              (if (`KismetMathLibrary.RandomBoolWithWeight` 0.3)
                (goto _label_6)
                (else
                  (`self.EndAttackCombo`))))
            (:`then_1`
              (`/Engine/EditorBlueprintResources/StandardMacros.IsValid` _target
                (:`Is Valid`
                  (`KismetSystemLibrary.Delay` 0.3)
                  (set `self.TargetPreLocation` (`self.K2_GetActorLocation` _target))
                  (bind (_direction _alpha) (`Timeline|JumpToTarget` :!via `PlayFromStart`)
                    (:`Update`
                      (`self.K2_SetActorLocation` (`KismetMathLibrary.VLerp` (`self.K2_GetActorLocation`) (+ (`self.TargetPreLocation`) (* (`self.GetActorForwardVector`) (`self.MinusOne`) (`self.JumpAttackLandDistance`))) _alpha)))))))))))))

(event `EndAttackCombo`
  ;[1 1 1] Attack Combo
  ;;[1 1 1] End Attack Combo
  (bind _result (`/Engine/EditorBlueprintResources/StandardMacros.DecrementInt` (`self.AttackCounts`))
    (:`  `
      (set `self.AttackCounts` _result)
      (set `self.Damage Type Class` "/Game/CombatSystem/Blueprints/DamageTypes/BP_AttackDamageType.BP_AttackDamageType_C")
      (`self.RotateToPlayer`))))

(event `QuickRotation`
  (bind (_returnvalue_roll _returnvalue_pitch _returnvalue_yaw) (`KismetMathLibrary.BreakRotator` (`self.K2_GetActorRotation`)))
  ;[1 1 1] Attack Combo
  ;;[1 1 1] Quick Rotate to player
  (bind (_direction _alpha) (`Timeline|ShortRotation` :!via `PlayFromStart` :!label _label_7)
    (:`Update`
      (bind _target (`self.Target`)
        (:`then`
          (bind (_returnvalue_roll_2 _returnvalue_pitch_2 _returnvalue_yaw_2) (`KismetMathLibrary.BreakRotator` (`KismetMathLibrary.FindLookAtRotation` (`self.K2_GetActorLocation`) (`self.K2_GetActorLocation` _target))))
          (bind (_returnvalue_roll_3 _returnvalue_pitch_3 _returnvalue_yaw_3) (`KismetMathLibrary.BreakRotator` (`KismetMathLibrary.RLerp` (`KismetMathLibrary.MakeRotator` 0.0 0.0 _returnvalue_yaw) (`KismetMathLibrary.MakeRotator` 0.0 0.0 _returnvalue_yaw_2) _alpha true)))
          (`self.K2_SetActorRotation` (`KismetMathLibrary.MakeRotator` 0.0 0.0 _returnvalue_yaw_3)))
        (:`else`
          (goto _label_7 :!via `Stop`))))))

(event `RotateToPlayer`
  (bind (_returnvalue_roll _returnvalue_pitch _returnvalue_yaw) (`KismetMathLibrary.BreakRotator` (`self.K2_GetActorRotation`)))
  ;[1 1 1] Rotate to player if relative angle is over 30
  (`self.GeneralCheck`
    (:`Can`
      (`self.Target`
        (:`then`
          (bind (_rotationtime _bneedtorotate) (`self.TurnInPlace`))
          (if _bneedtorotate
            (`TimelineComponent.SetPlayRate` (`self.RotateCurve`) (/ 1.0 (select `bool` (`KismetMathLibrary.NearlyEqual_FloatFloat` _rotationtime) :`false` _rotationtime :`true` 1.0)))
            (bind (_direction _alpha) (`Timeline|RotateCurve` :!via `PlayFromStart` :!label _label_8)
              (:`Update`
                (bind _target (`self.Target`)
                  (:`then`
                    (bind (_returnvalue_roll_2 _returnvalue_pitch_2 _returnvalue_yaw_2) (`KismetMathLibrary.BreakRotator` (`KismetMathLibrary.FindLookAtRotation` (`self.K2_GetActorLocation`) (`self.K2_GetActorLocation` _target))))
                    (bind (_returnvalue_roll_3 _returnvalue_pitch_3 _returnvalue_yaw_3) (`KismetMathLibrary.BreakRotator` (`KismetMathLibrary.RLerp` (`KismetMathLibrary.MakeRotator` 0.0 0.0 _returnvalue_yaw) (`KismetMathLibrary.MakeRotator` 0.0 0.0 _returnvalue_yaw_2) _alpha true)))
                    (`self.K2_SetActorRotation` (`KismetMathLibrary.MakeRotator` 0.0 0.0 _returnvalue_yaw_3)))
                  (:`else`
                    (goto _label_8 :!via `Stop`))))
              (:`Finished`
                (`self.GeneralCheck` :!label _label_9
                  (:`Can`
                    (set `self.bEnableTick` true)
                    (`self.NextAttack`)))))
            (else
              (goto _label_9))))
        (:`else`)))))

(event `self.CapsuleComponent.OnComponentHit`
  (params (HitComponent :type "PrimitiveComponent Object Reference") (OtherActor :type "Actor Object Reference") (OtherComp :type "PrimitiveComponent Object Reference") (NormalImpulse :type "Vector Structure") (Hit :type "HitResult Structure (by ref)"))
  ;[1 1 1] CollisionCheck
  (if (`self.bIsStrafing`)
    (`/Engine/EditorBlueprintResources/StandardMacros.DoOnce` false :!label _label_10
      (:`Completed`
        (bind (_outhit _returnvalue) (`KismetSystemLibrary.BoxTraceSingleForObjects` (`self.K2_GetActorLocation`) (select `/Game/CombatSystem/Blueprints/AI/Enums/E_AIMovementDirections` (`self.AIMovementDirections`) :`NewEnumerator2` (+ (`self.K2_GetActorLocation`) (* (* (`self.GetActorForwardVector`) (`self.MinusOne`)) (`self.CollisionCheckDistance`))) :`NewEnumerator3` (+ (`self.K2_GetActorLocation`) (* (* (`self.GetActorRightVector`) (`self.MinusOne`)) (`self.CollisionCheckDistance`))) :`NewEnumerator4` (+ (`self.K2_GetActorLocation`) (* (`self.GetActorRightVector`) (`self.CollisionCheckDistance`)))) (50.0 50.0 50.0) (struct) (`|MakeArray` "ObjectTypeQuery1" "ObjectTypeQuery3" :!type "EObjectTypeQuery Enum")))
        (if _returnvalue
          (set `self.IsColliding` true)
          (`self.StartStrafe`)
          (`KismetSystemLibrary.Delay` 0.2)
          (goto _label_10 :!via `Reset`))))))

(fn `PerformStun`
  (returns (bIsSuccessful :type Boolean))
  (set `self.bEnableTick` false)
  (set `self.bAllowBehave` false)
  (bind _bissuccessful (`parent.PerformStun`))
  (return _bissuccessful))

(fn `TurnInPlace`
  (returns (RotationTime :type "Float (double-precision)") (bNeedToRotate :type Boolean))
  (locals (`L_RelativeRotation]` :type "Float (double-precision)") (L_RotationTime :type "Float (single-precision)" :default 0.0))
  (bind (_returnvalue_roll _returnvalue_pitch _returnvalue_yaw) (`KismetMathLibrary.BreakRotator` (`self.K2_GetActorRotation`)))
  (bind _l_relativerotation_ (`local.L_RelativeRotation]`))
  (bind _l_relativerotation__2 (`local.L_RelativeRotation]`))
  (bind _l_relativerotation__3 (`local.L_RelativeRotation]`))
  (bind _l_relativerotation__4 (`local.L_RelativeRotation]`))
  (bind _l_relativerotation__5 (`local.L_RelativeRotation]`))
  (bind _l_relativerotation__6 (`local.L_RelativeRotation]`))
  (bind _target (`self.Target`)
    (:`then`
      (bind (_returnvalue_roll_2 _returnvalue_pitch_2 _returnvalue_yaw_2) (`KismetMathLibrary.BreakRotator` (`KismetMathLibrary.FindLookAtRotation` (`self.K2_GetActorLocation`) (`self.K2_GetActorLocation` _target))))
      (set `local.L_RelativeRotation]` (- _returnvalue_yaw_2 _returnvalue_yaw))
      ;[1 1 1 1 14] Play only if absolute value over 30
      (if true
        (return 0.0 false)
        (else
          (if (or (and (> _l_relativerotation_ 0.0) (<= _l_relativerotation_ 90.0)) (and (< _l_relativerotation__2 -360.0) (>= _l_relativerotation__2 -270.0)))
            (`KismetSystemLibrary.PrintString` "Player is right forward of enemy")
            (bind _returnvalue (`self.PlayAnimMontage` "/Game/CombatSystem/CourseFiles/Animations/TurnInPlace/Turn_Right_90_Montage.Turn_Right_90_Montage"))
            (set `local.L_RotationTime` _returnvalue)
            (elif (or (and (> _l_relativerotation__3 90.0) (<= _l_relativerotation__3 180.0)) (and (< _l_relativerotation__4 -270.0) (>= _l_relativerotation__4 -180.0)))
              (`KismetSystemLibrary.PrintString` "Player right backward")
              (bind _returnvalue_2 (`self.PlayAnimMontage` "/Game/CombatSystem/CourseFiles/Animations/TurnInPlace/Turn_Right_180_Montage.Turn_Right_180_Montage"))
              (set `local.L_RotationTime` _returnvalue_2)
              (elif (or (and (> _l_relativerotation__5 180.0) (<= _l_relativerotation__5 270.0)) (and (< _l_relativerotation__6 -180.0) (>= _l_relativerotation__6 -90.0)))
                (`KismetSystemLibrary.PrintString` "Player left backward")
                (bind _returnvalue_3 (`self.PlayAnimMontage` "/Game/CombatSystem/CourseFiles/Animations/TurnInPlace/Turn_Left_180_Montage.Turn_Left_180_Montage"))
                (set `local.L_RotationTime` _returnvalue_3)
                (else
                  (`KismetSystemLibrary.PrintString` "Player left forward")
                  (bind _returnvalue_4 (`self.PlayAnimMontage` "/Game/CombatSystem/CourseFiles/Animations/TurnInPlace/Turn_Left_90_Montage.Turn_Left_90_Montage"))
                  (set `local.L_RotationTime` _returnvalue_4)))))
          (return (`local.L_RotationTime`) true))))
    (:`else`)))

(fn `UserConstructionScript`
  (`parent.UserConstructionScript`))