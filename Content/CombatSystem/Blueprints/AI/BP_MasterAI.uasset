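; Master AI character for melee combat, coordinating stats, gameplay-tag state, combat and weapon collision components.
; Point damage feeds stats and AI damage sensing, then triggers impact effects and front/back stun or knockdown montages chosen by dot product.
; Attacks and actions play tag-selected montages, with combo indexing and timeline-driven rotation toward the target.
; Death stops AI logic, sets a blackboard flag, plays a montage or ragdolls, then destroys the actor.
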(event `self.ReceiveBeginPlay`
  ;[1 1 1] Initialize Stats
  (`/Game/CombatSystem/Blueprints/Components/BP_StatsComponent.InitializeStats` (`self.StatsComponent`)))

(event `self.ReceivePointDamage`
  (params (Damage :type "Float (single-precision)") (DamageType :type "DamageType Object Reference") (HitLocation :type "Vector Structure") (HitNormal :type "Vector Structure") (HitComponent :type "PrimitiveComponent Object Reference") (BoneName :type Name) (ShotFromDirection :type "Vector Structure") (InstigatedBy :type "Controller Object Reference") (DamageCauser :type "Actor Object Reference") (HitInfo :type "HitResult Structure (by ref)"))
  (bind _returnvalue (`Controller.K2_GetPawn` InstigatedBy))
  ;[1 0 0] Point Damage Event
  (bind _asbp_attack_damage_type (cast `/Game/CombatSystem/Blueprints/DamageTypes/BP_AttackDamageType` DamageType))
  (`/Game/CombatSystem/Blueprints/Components/BP_StatsComponent.TakeDamage` (`self.StatsComponent`) Damage)
  (`AISense_Damage.ReportDamageEvent` self _returnvalue Damage HitLocation HitLocation)
  (set `self.bIsHitFront` (`KismetMathLibrary.InRange_FloatFloat` (`self.GetDotProductTo` self _returnvalue) -0.1))
  (set `self.LastHitInfo` HitInfo)
  (bind _damagetype (`/Game/CombatSystem/Blueprints/DamageTypes/BP_AttackDamageType.DamageType` _asbp_attack_damage_type))
  (`self.ApplyImpactEffect` _damagetype)
  (if (`self.CanReceiveHitReaction`)
    (`self.ApplyHitReaction` _damagetype)))

(event `/Game/CombatSystem/Blueprints/Interfaces/Targeting_BPI.OnTargeted`
  (params (bIsTargeted :type Boolean))
  ;[1 1 1] Lock-On Target Dot
  (`SceneComponent.SetVisibility` (`self.TargetingDotWidget`) bIsTargeted false))

(event `AttackEvent`
  ;[1 1 1] Attacking
  ;;[1 0 0] Attack Event
  (if (`self.CanPerformAttack`)
    (`self.PerformAttack` (`self.GetDesiredAttackType`) (`/Game/CombatSystem/Blueprints/Components/BP_CombatComponent.AttackCount` (`self.CombatComponent`)))))

(event `self.StatsComponent.OnCurrentStatValueUpdated`
  (params (StatType :type "/Game/CombatSystem/Blueprints/Enums/E_Stats Enum" :default "NewEnumerator0") (Value :type "Float (double-precision)"))
  ;[1 1 1] Perform death via Health stat
  (if (and (`|EnumEquality` StatType "NewEnumerator1") (<= Value 0.0))
    (`self.PerformDeath`)))

(event `ApplyHitReaction`
  (params (InDamageType :type "/Game/CombatSystem/Blueprints/Enums/E_DamageType Enum" :default "NewEnumerator0"))
  ;[1 0 0] Apply Hit Reaction
  (switch `/Game/CombatSystem/Blueprints/Enums/E_DamageType` "NewEnumerator0"
    (:`NewEnumerator0`
      (`self.PerformHitStun` :!label _label))
    (:`NewEnumerator1`
      (goto _label))
    (:`NewEnumerator2`
      (`self.PerformKnockdown`))))

(event `self.SetIFrames`
  (params (bEnableIFrames :type Boolean))
  ;[1 1 1] Set Iframes
  (set `self.bIsFramesEnabled` bEnableIFrames))

(event `self.ContinueAttack`
  ;[1 1 1] Attacking
  ;;[1 0 0] Continue Attack Event
  (if (`/Game/CombatSystem/Blueprints/Components/BP_CombatComponent.bIsAttackSaved` (`self.CombatComponent`))
    (set `/Game/CombatSystem/Blueprints/Components/BP_CombatComponent.bIsAttackSaved` false (`self.CombatComponent`))
    (if (== (`/Game/CombatSystem/Blueprints/Components/BP_StateManagerComponent.GetCurrentState` (`self.StateManagerComponent`)) (struct :`TagName` "Character.State.Attacking"))
      (`/Game/CombatSystem/Blueprints/Components/BP_StateManagerComponent.SetCurrentState` :`self` (`self.StateManagerComponent`)))
    (`self.AttackEvent`)))

(event `ApplyImpactEffect`
  (params (InDamageType :type "/Game/CombatSystem/Blueprints/Enums/E_DamageType Enum" :default "NewEnumerator0"))
  (bind (_bblockinghit _binitialoverlap _time _distance _location) (`GameplayStatics.BreakHitResult` (`self.LastHitInfo`)))
  ;[1 0 0] Apply Impact Event
  (switch `/Game/CombatSystem/Blueprints/Enums/E_DamageType` "NewEnumerator0"
    (:`NewEnumerator0`
      _)
    (:`NewEnumerator1`
      _)
    (:`NewEnumerator2`
      _))
  (`GameplayStatics.PlaySoundAtLocation` (`self.ImpactSound`) _location (struct) 1.0 1.0 0.0 null null null null)
  (`GameplayStatics.SpawnEmitterAtLocation` (`self.ImpactEffect`) _location))

(event `self.ResetAttack`
  ;[1 1 1] Attacking
  (`/Game/CombatSystem/Blueprints/Components/BP_CombatComponent.ResetAttack` (`self.CombatComponent`)))

(event `self.ResetCombat`
  ;[1 1 1] Attacking
  ;;[1 0 0] Reset Combat
  (`/Game/CombatSystem/Blueprints/Components/BP_CombatComponent.ResetAttack` (`self.CombatComponent`))
  (`/Game/CombatSystem/Blueprints/Components/BP_StateManagerComponent.ResetState` (`self.StateManagerComponent`))
  (`/Game/CombatSystem/Blueprints/Components/BP_StateManagerComponent.ResetAction` (`self.StateManagerComponent`)))

(event `self.RotateToTarget`
  ;[1 1 1] Rotate To Target
  (`self.StartRotateTimeline`))

(event `OnTargetSet`
  (params (NewTarget :type "Actor Object Reference"))
  ;[1 1 1] On Target Set
  ;[1 0 0] Character States
  (set `self.TargetActor` NewTarget))

(event `self.StateManagerComponent.OnStateBegin`
  (params (CharacterState :type "GameplayTag Structure"))
  ;[1 0 0] Character States
  (`|SwitchGameplayTag` CharacterState
    (:`Character.State.Dead`
      (`self.PerformDeath`))))

(event `self.ActivateCollision`
  (params (CollisionPart :type "/Game/CombatSystem/Blueprints/Enums/ECollisionPart Enum" :default "NewEnumerator0"))
  ;[1 1 1] Activate/Deactivate Collisions
  (switch `/Game/CombatSystem/Blueprints/Enums/ECollisionPart` CollisionPart
    (:`NewEnumerator0`
      (`/Game/CombatSystem/Blueprints/Components/BP_CollisionComponent.ActivateCollision` (`self.MainWeaponCollisionComponent`)))
    (:`NewEnumerator1`
      (`/Game/CombatSystem/Blueprints/Components/BP_CollisionComponent.ActivateCollision` (`self.OffhandWeaponCollisionComponent`)))))

(event `StartRotateTimeline`
  (bind _returnvalue (`self.K2_GetActorRotation`))
  (bind (_returnvalue_roll _returnvalue_pitch _returnvalue_yaw) (`KismetMathLibrary.BreakRotator` (`KismetMathLibrary.RInterpTo` _returnvalue (`KismetMathLibrary.FindLookAtRotation` (`self.K2_GetActorLocation`) (`self.K2_GetActorLocation` (`self.TargetActor`))) (`GameplayStatics.GetWorldDeltaSeconds`) 9.0)))
  ;[1 1 1] Rotate To Target
  (`Timeline|RotateToTargetTL` :!label _label_2
    (:`Update`
      (`/Engine/EditorBlueprintResources/StandardMacros.IsValid` (`self.TargetActor`)
        (:`Is Valid`
          (`self.K2_SetActorRotation` (`KismetMathLibrary.MakeRotator` (.roll _returnvalue) (.pitch _returnvalue) _returnvalue_yaw)))))))

(event `StopRotatingToTarget`
  ;[1 1 1] Rotate To Target
  (goto _label_2 :!via `Stop`))

(event `self.CombatComponent.OnCombatToggled`
  (params (bIsCombatEnabled :type Boolean))
  ;[1 1 1] Toggle Combat Enabled
)

(event `self.DeactivateCollision`
  (params (CollisionPart :type "/Game/CombatSystem/Blueprints/Enums/ECollisionPart Enum" :default "NewEnumerator0"))
  ;[1 1 1] Activate/Deactivate Collisions
  (switch `/Game/CombatSystem/Blueprints/Enums/ECollisionPart` CollisionPart
    (:`NewEnumerator0`
      (`/Game/CombatSystem/Blueprints/Components/BP_CollisionComponent.DeactivateCollision` (`self.MainWeaponCollisionComponent`)))))

(event `self.StateManagerComponent.OnStateEnd`
  (params (CharacterState :type "GameplayTag Structure"))
  ;[1 0 0] Character States
  (`|SwitchGameplayTag` CharacterState
    (:`Character.State.Attacking`
      (`self.StopRotatingToTarget`))))

(event `PerformDeath`
  ;[1 0 0] Character States
  ;;[1 1 1] Perform Death
  (if (not (`self.GetIsDead`))
    (`self.SetIsDead` true)
    (`BrainComponent.StopLogic` (`AIController.BrainComponent` (`AIBlueprintHelperLibrary.GetAIController` self)) "Dead")
    (if (`KismetArrayLibrary.Array_IsNotEmpty` (`self.DeathAnimation`))
      (`self.PlayAnimMontage` (`KismetArrayLibrary.Array_Random` (`self.DeathAnimation`)))
      (else
        (`self.EnableRagdoll`)))
    (`self.ApplyHitReactionPhysicsVelocity` (`KismetMathLibrary.SelectFloat` 2000.0 -2000.0 (`self.bIsHitFront`)))
    (`PrimitiveComponent.SetCollisionResponseToChannel` (`self.CapsuleComponent`) "ECC_Pawn" "ECR_Overlap")
    (`KismetSystemLibrary.Delay` 4.0)
    (`self.K2_DestroyActor`)))

(fn `ApplyHitReactionPhysicsVelocity`
  (params (InitialSpeed :type "Float (double-precision)"))
  (`PrimitiveComponent.SetPhysicsLinearVelocity` (`self.Mesh`) (* (`self.GetActorForwardVector`) (* (`local.InitialSpeed`) -1.0)) false (`self.PelvisBoneName`)))

(fn `CanBeTargeted`
  (returns (ReturnValue :type Boolean))
  (return (!= (`/Game/CombatSystem/Blueprints/Components/BP_StateManagerComponent.GetCurrentState` (`self.StateManagerComponent`)) (struct :`TagName` "Character.State.Dead"))))

(fn `CanPerformAttack`
  (returns (ReturnValue :type Boolean))
  (return (and (not (`/Game/CombatSystem/Blueprints/Components/BP_StateManagerComponent.IsCurrentStateEqualToAny` (`self.StateManagerComponent`) (struct :`GameplayTags` (struct :`(TagName` "Character.State.Attacking") :`(TagName` "Character.State.Dead") :`(TagName` "Character.State.Disabled") :`(TagName` "Character.State.Dodging") :`(TagName` "Character.State.General Action State"))))) (>= (`/Game/CombatSystem/Blueprints/Components/BP_StatsComponent.GetCurrentStatValue` (`self.StatsComponent`) "NewEnumerator2") 10.0) (`/Game/CombatSystem/Blueprints/Components/BP_CombatComponent.GetIsCombatEnabled` (`self.CombatComponent`)))))

(fn `CanPerformDodge`
  (returns (ReturnValue :type Boolean))
  (return (and (not (`/Game/CombatSystem/Blueprints/Components/BP_StateManagerComponent.IsCurrentStateEqualToAny` (`self.StateManagerComponent`) (struct :`GameplayTags` (struct :`(TagName` "Character.State.Dead") :`(TagName` "Character.State.Disabled") :`(TagName` "Character.State.Dodging") :`(TagName` "Character.State.General Action State"))))) (not (`NavMovementComponent.IsFalling` (`self.CharacterMovement`))) (>= (`/Game/CombatSystem/Blueprints/Components/BP_StatsComponent.GetCurrentStatValue` (`self.StatsComponent`) "NewEnumerator2") 10.0))))

(fn `CanPerformJump`
  (returns (ReturnValue :type Boolean))
  (return (and (not (`/Game/CombatSystem/Blueprints/Components/BP_StateManagerComponent.IsCurrentStateEqualToAny` (`self.StateManagerComponent`) (struct :`GameplayTags` (struct :`(TagName` "Character.State.Dead") :`(TagName` "Character.State.Disabled") :`(TagName` "Character.State.Dodging") :`(TagName` "Character.State.General Action State"))))) (not (`NavMovementComponent.IsFalling` (`self.CharacterMovement`))))))

(fn `CanPerformSprint`
  (returns (ReturnValue :type Boolean))
  (return (!= (`KismetMathLibrary.VSize` (`self.GetVelocity`)) 0.0)))

(fn `CanPerformToggleCombat`
  (returns (ReturnValue :type Boolean))
  (return (and (not (`/Game/CombatSystem/Blueprints/Components/BP_StateManagerComponent.IsCurrentStateEqualToAny` (`self.StateManagerComponent`) (struct :`GameplayTags` (struct :`(TagName` "Character.State.Attacking") :`(TagName` "Character.State.Dead") :`(TagName` "Character.State.Disabled") :`(TagName` "Character.State.Dodging") :`(TagName` "Character.State.General Action State"))))) (not (`NavMovementComponent.IsFalling` (`self.CharacterMovement`))))))

(fn `CanReceiveDamage`
  (returns (ReturnValue :type Boolean))
  (return (and (not (`/Game/CombatSystem/Blueprints/Components/BP_StateManagerComponent.IsCurrentStateEqualToAny` (`self.StateManagerComponent`) (struct :`GameplayTags` (struct :`(TagName` "Character.State.Dead"))))) (not (`self.bIsFramesEnabled`)))))

(fn `CanReceiveHitReaction`
  (returns (ReturnValue :type Boolean))
  (return (and (not (`/Game/CombatSystem/Blueprints/Components/BP_StateManagerComponent.IsCurrentStateEqualToAny` (`self.StateManagerComponent`) (struct :`GameplayTags` (struct :`(TagName` "Character.State.Dead"))))) (not (`self.GetIsDead`)))))

(fn `EnableRagdoll`
  (bind _pelvisbonename (`self.PelvisBoneName`))
  ;[1 1 1] Create Ragdoll effect with simulated physics
  (`CharacterMovementComponent.SetMovementMode` (`self.CharacterMovement`) "MOVE_None" 0)
  (`PrimitiveComponent.SetCollisionResponseToChannel` (`self.CapsuleComponent`) "ECC_Pawn" "ECR_Ignore")
  (`PrimitiveComponent.SetCollisionResponseToChannel` (`self.CapsuleComponent`) "ECC_Camera" "ECR_Ignore")
  (`PrimitiveComponent.SetCollisionProfileName` (`self.Mesh`) "ragdoll" true)
  (`SkeletalMeshComponent.SetAllBodiesBelowSimulatePhysics` (`self.Mesh`) _pelvisbonename true true)
  (`SkeletalMeshComponent.SetAllBodiesBelowPhysicsBlendWeight` (`self.Mesh`) _pelvisbonename 1.0 false true))

(fn `GetActionMontage`
  (params (ActionTag :type "GameplayTag Structure"))
  (returns (Montages :type "Array of AnimMontage Object Reference"))
  (`|SwitchGameplayTag` ActionTag
    (:`Character.Action.Attack.Close Range`
      (return (`self.CloseRangeAttackMontages`)))
    (:`Character.Action.Attack.Medium Range`
      (return (`self.MediumRangeAttackMontages`)))
    (:`Character.Action.Attack.Rare Attack`
      (return (`self.RareAttackMontages`)))
    (:`Character.Action.Dodge`
      (return (`self.Dodge Montages`)))
    (:`Character.Action.Enter Combat`
      (return (`|MakeArray` (`self.Enter Combat`))))
    (:`Character.Action.Exit Combat`
      (return (`|MakeArray` (`self.ExitCombat`))))
    (:`Character.Action.Intro`
      (return (`self.Intro Montages`)))))

(fn `GetCurrentSpeedMode`
  (returns (ReturnValue :type "/Game/CombatSystem/Blueprints/Enums/E_MovementSpeedMode Enum"))
  (return (`self.MovementSpeedMode`)))

(fn `GetDesiredAttackType`
  (returns (ReturnValue :type "GameplayTag Structure"))
  (if (`NavMovementComponent.IsFalling` (`self.CharacterMovement`))
    (return (struct :`TagName` "Character.Action.Attack.Falling Attack"))
    (elif (`|EnumEquality` (`self.GetCurrentSpeedMode`) "NewEnumerator2")
      (return (struct :`TagName` "Character.Action.Attack.Sprinting Attack"))
      (else
        (return (struct :`TagName` "Character.Action.Attack.Light Attack"))))))

(fn `GetDesiredRotation`
  (returns (ReturnValue :type "Rotator Structure"))
  (if (!= (`PawnMovementComponent.GetLastInputVector` (`self.CharacterMovement`)) (0.0 0.0 0.0) :`ErrorTolerance` 0.001)
    ;[1 1 1] If Character moving, return last input rotation
    (return (`KismetMathLibrary.Conv_VectorToRotator` (`self.GetLastMovementInputVector`)))
    (else
      ;[1 1 1] If character not moving, get current rotation
      (return (`self.K2_GetActorRotation`)))))

(fn `GetIsDead`
  (returns (ReturnValue :type Boolean))
  (return (`self.bIsDead`)))

(fn `GetMovementSpeedMode`
  (returns (ReturnValue :type "/Game/CombatSystem/Blueprints/Enums/E_MovementSpeedMode Enum"))
  (return (`self.GetCurrentSpeedMode`)))

(fn `GetOwnedGameplayTags`
  (returns (ReturnValue :type "GameplayTagContainer Structure"))
  (return (`self.OwnedGameplayTags`)))

(fn `GetWeaponMesh`
  (returns (ReturnValue :type "PrimitiveComponent Object Reference"))
  (return null))

(fn `HasMatchingGameplayTag`
  (params (TagToCheck :type "GameplayTag Structure"))
  (returns (ReturnValue :type Boolean))
  (return (`BlueprintGameplayTagLibrary.HasTag` (`self.OwnedGameplayTags`) TagToCheck)))

(fn `PerformAction`
  (params (ActionTag :type "GameplayTag Structure") (StateTag :type "GameplayTag Structure") (MontageIndex :type Integer) (bRandomIndex :type Boolean))
  (returns (IsSuccess :type Boolean) (ActionDuration :type "Float (double-precision)"))
  (locals (L_ActionMontages :type "Array of AnimMontage Object Reference") (L_ActionMontage :type "AnimMontage Object Reference"))
  (bind _l_actionmontages (`local.L_ActionMontages`))
  (set `local.L_ActionMontages` (`self.GetActionMontage` ActionTag))
  (bind _output_get (set `local.L_ActionMontage` (select `bool` (`local.bRandomIndex`) :`false` (`|GetArrayItem` _l_actionmontages (`KismetMathLibrary.SelectInt` (`local.MontageIndex`) 0 (> (`local.MontageIndex`) (`KismetArrayLibrary.Array_LastIndex` (`local.L_ActionMontages`))))) :`true` (`KismetArrayLibrary.Array_Random` _l_actionmontages))))
  (`/Engine/EditorBlueprintResources/StandardMacros.IsValid` _output_get
    (:`Is Valid`
      (`/Game/CombatSystem/Blueprints/Components/BP_StateManagerComponent.SetCurrentState` (`self.StateManagerComponent`) (`local.StateTag`))
      (`/Game/CombatSystem/Blueprints/Components/BP_StateManagerComponent.SetCurrentAction` (`self.StateManagerComponent`) (`local.ActionTag`))
      (bind _returnvalue (`AnimInstance.Montage_Play` (`SkeletalMeshComponent.GetAnimInstance` (`self.Mesh`)) (`local.L_ActionMontage`) 1.0 "Duration" 0.0 true))
      (return true _returnvalue))
    (:`Is Not Valid`
      (`KismetSystemLibrary.PrintString` (`KismetStringLibrary.Concat_StrStr` "Index" (`KismetStringLibrary.Conv_IntToString` (`local.MontageIndex`)) "NOT IN INDEX") true true (struct :`R` 1.0 :`G` 0.031575 :`B` 0.087313 :`A` 1.0))
      (return false 0.0))))

(fn `PerformAttack`
  (params (AttackType :type "GameplayTag Structure") (AttackIndex :type Integer) (bRandomIndex :type Boolean))
  (returns (IsSuccess :type Boolean) (AttackDuration :type "Float (double-precision)"))
  (locals (L_AttackMontages :type "Array of AnimMontage Object Reference") (L_AttackMontage :type "AnimMontage Object Reference") (L_AttackDuration :type "Float (single-precision)" :default 0.0))
  (bind _l_attackmontages (`local.L_AttackMontages`))
  (bind _attackindex (`local.AttackIndex`))
  ;[1 1 1] Perform attack montage from array of available attacks by index or random, set is attacking true and play animation, increment through attack array
  (set `local.L_AttackMontages` (`self.GetActionMontage` AttackType))
  (bind _output_get (set `local.L_AttackMontage` (select `bool` (`local.bRandomIndex`) :`false` (`|GetArrayItem` _l_attackmontages (select `bool` (> _attackindex (`KismetArrayLibrary.Array_LastIndex` (`local.L_AttackMontages`))) :`false` _attackindex)) :`true` (`KismetArrayLibrary.Array_Random` _l_attackmontages))))
  (`/Engine/EditorBlueprintResources/StandardMacros.IsValid` _output_get
    (:`Is Valid`
      (`/Game/CombatSystem/Blueprints/Components/BP_StateManagerComponent.SetCurrentState` (`self.StateManagerComponent`) (struct :`TagName` "Character.State.Attacking"))
      (`/Game/CombatSystem/Blueprints/Components/BP_StateManagerComponent.SetCurrentAction` (`self.StateManagerComponent`) (`local.AttackType`))
      (bind _returnvalue (`AnimInstance.Montage_Play` (`SkeletalMeshComponent.GetAnimInstance` (`self.Mesh`)) (`local.L_AttackMontage`) 1.0 "Duration" 0.0 true))
      (set `local.L_AttackDuration` _returnvalue)
      ;[1 1 1] Reset attack inrement to 0 index when max index reached return attack duration
      (bind _result (`/Engine/EditorBlueprintResources/StandardMacros.IncrementInt` (`/Game/CombatSystem/Blueprints/Components/BP_CombatComponent.AttackCount` (`self.CombatComponent`)))
        (:`  `
          (if (> _result (`KismetArrayLibrary.Array_LastIndex` (`local.L_AttackMontages`)))
            (set `/Game/CombatSystem/Blueprints/Components/BP_CombatComponent.AttackCount` 0 (`self.CombatComponent`)))
          (return false (`local.L_AttackDuration`)))))
    (:`Is Not Valid`
      (`KismetSystemLibrary.PrintString` "Not in Index" true true (struct :`R` 1.0 :`G` 0.031575 :`B` 0.087313 :`A` 1.0))
      (return false 0.0))))

(fn `PerformCustomAction`
  (params (ActionTag :type "GameplayTag Structure") (StateTag :type "GameplayTag Structure") (InMontgae :type "AnimMontage Object Reference") (MontagePlayRate :type "Float (double-precision)") (bAutoReset :type Boolean))
  (returns (bIsSuccess :type Boolean))
  (return false))

(fn `PerformHitStun`
  (returns (bIsSuccessful :type Boolean))
  (locals (L_HitMontage :type "AnimMontage Object Reference"))
  ;[1 1 1] Checks if front or back attack, plays appropriate montage and sets state to disabled
  (bind _output_get (set `local.L_HitMontage` (select `bool` (`self.bIsHitFront`) :`false` (`self.HitStunBackMontage`) :`true` (`self.HitStunFrontMontage`))))
  (`/Engine/EditorBlueprintResources/StandardMacros.IsValid` _output_get
    (:`Is Valid`
      (`/Game/CombatSystem/Blueprints/Components/BP_StateManagerComponent.SetCurrentState` (`self.StateManagerComponent`) (struct :`TagName` "Character.State.Disabled"))
      (`self.PlayAnimMontage` (`local.L_HitMontage`))
      (return true))
    (:`Is Not Valid`
      (return false))))

(fn `PerformKnockdown`
  (returns (bIsSuccessful :type Boolean))
  (locals (L_HitMontage :type "AnimMontage Object Reference"))
  ;[1 1 1] Checks if front or back attack, plays appropriate montage and sets state to disabled
  (bind _output_get (set `local.L_HitMontage` (select `bool` (`self.bIsHitFront`) :`false` (`self.KnockdownBackMontage`) :`true` (`self.KnockdownFrontMontage`))))
  (`/Engine/EditorBlueprintResources/StandardMacros.IsValid` _output_get
    (:`Is Valid`
      (`/Game/CombatSystem/Blueprints/Components/BP_StateManagerComponent.SetCurrentState` (`self.StateManagerComponent`) (struct :`TagName` "Character.State.Disabled"))
      (`self.PlayAnimMontage` (`local.L_HitMontage`))
      (return true))
    (:`Is Not Valid`
      (return false))))

(fn `SetIsDead`
  (params (bCondition :type Boolean))
  (if (!= bCondition (`self.bIsDead`))
    (bind _output_get (set `self.bIsDead` bCondition))
    (`BlackboardComponent.SetValueAsBool` (`AIBlueprintHelperLibrary.GetBlackboard` (`AIBlueprintHelperLibrary.GetAIController` self)) "bIsDead" _output_get)))

(fn `SetMovementSpeedMode`
  (params (NewSpeedMode :type "/Game/CombatSystem/Blueprints/Enums/E_MovementSpeedMode Enum" :default "NewEnumerator0"))
  ;[1 1 1] set walk speed value to movement mode value
  (if (`|EnumInequality` NewSpeedMode (`self.MovementSpeedMode`))
    (bind _output_get (set `self.MovementSpeedMode` (`local.NewSpeedMode`)))
    (switch `/Game/CombatSystem/Blueprints/Enums/E_MovementSpeedMode` _output_get
      (:`NewEnumerator0`
        (set `CharacterMovementComponent.MaxWalkSpeed` (`self.WalkingSpeed`) (`self.CharacterMovement`)))
      (:`NewEnumerator1`
        (set `CharacterMovementComponent.MaxWalkSpeed` (`self.JoggingSpeed`) (`self.CharacterMovement`)))
      (:`NewEnumerator2`
        (set `CharacterMovementComponent.MaxWalkSpeed` (`self.SprintingSpeed`) (`self.CharacterMovement`))))))

(fn `UseItemByTag`
  (params (ItemTag :type "GameplayTag Structure"))
  (returns (bIsSuccess :type Boolean))
  (return false))

(fn `UserConstructionScript`)