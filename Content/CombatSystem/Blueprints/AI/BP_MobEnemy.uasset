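; Mob enemy Blueprint that adds weapon combat and a targeting health bar on top of its parent's behavior.
; Weapon collision hits apply point damage from a StatsComponent value to actors that can receive it.
; A health bar widget reads the same stats and shows only while targeted.
; Combat toggling moves the weapon between sockets, and death switches it to PhysicsActor collision with simulation left off.
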(event `self.ReceiveBeginPlay`
  ;[1 0 0] Begin Play
  (`parent.ReceiveBeginPlay`)
  (`/Game/CombatSystem/Blueprints/Components/BP_CollisionComponent.SetCollisionMeshComponent` (`self.MainWeaponCollisionComponent`) (`self.GetWeaponMesh`))
  (bind _returnvalue (`|CreateWidget` "/Game/CombatSystem/UI/WB_HealthBar.WB_HealthBar_C" (`GameplayStatics.GetPlayerController` 0) (`self.StatsComponent`)))
  (`WidgetComponent.SetWidget` (`self.HealthBar`) _returnvalue))

(event `self.MainWeaponCollisionComponent.OnHit`
  (params (HitResult :type "HitResult Structure"))
  (bind (_bblockinghit _binitialoverlap _time _distance _location _impactpoint _normal _impactnormal _physmat _hitactor) (`GameplayStatics.BreakHitResult` HitResult))
  ;[1 1 1] On Hit Event
  (bind _returnvalue (message `/Game/CombatSystem/Blueprints/Interfaces/Combat_BPI.CanReceiveDamage` _hitactor))
  (if _returnvalue
    (`GameplayStatics.ApplyPointDamage` _hitactor (`/Game/CombatSystem/Blueprints/Components/BP_StatsComponent.GetCurrentStatValue` (`self.StatsComponent`) "NewEnumerator4") (`self.GetActorForwardVector`) HitResult (`self.GetController`) self "/Game/CombatSystem/Blueprints/DamageTypes/BP_AttackDamageType.BP_AttackDamageType_C")))

(event `/Game/CombatSystem/Blueprints/Interfaces/Targeting_BPI.OnTargeted`
  (params (bIsTargeted :type Boolean))
  ;[1 1 1] Targeting Event
  (`parent.OnTargeted` bIsTargeted)
  (`SceneComponent.SetVisibility` (`self.HealthBar`) bIsTargeted false))

(event `SimulateWeaponPhysics`
  (bind _returnvalue (`self.GetWeaponMesh`))
  ;[1 1 1] Simulate Physics
  (`PrimitiveComponent.SetCollisionProfileName` _returnvalue "PhysicsActor" true)
  (`PrimitiveComponent.SetSimulatePhysics` _returnvalue false))

(event `self.PerformDeath`
  ;[1 1 1] Perform Death
  (`parent.PerformDeath`)
  (`self.SimulateWeaponPhysics`))

(event `self.CombatComponent.OnCombatToggled`
  (params (bIsCombatEnabled :type Boolean))
  ;[1 1 1] Attach Weapon to sockets
  (`SceneComponent.K2_AttachToComponent` (`self.GetWeaponMesh`) (`self.Mesh`) (select `bool` bIsCombatEnabled :`false` (`self.AttachSocketName`) :`true` (`self.WeaponHandSocketName`)) "KeepRelative" "KeepRelative" "KeepRelative" true))

(fn `UserConstructionScript`
  (`parent.UserConstructionScript`))