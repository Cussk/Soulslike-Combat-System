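; Humanoid boss enemy Blueprint that adds a boss health bar and a melee weapon to its parent enemy behavior.
; BeginPlay creates the health widget from the StatsComponent, and target changes and death toggle its visibility.
; Weapon collision hits apply point damage from a current stat, while combat toggles move the weapon between hand and attach sockets.
; On death the weapon switches to the PhysicsActor profile, though physics simulation is set to false.
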(event `SetBossHealthVisibility`
  (params (bIsVisible :type Boolean))
  ;[1 1 1] Set Boss Health Visibility
  (bind _bosshealthui (`self.BossHealthUI`)
    (:`then`
      (`Widget.SetVisibility` _bosshealthui (select `bool` bIsVisible :`false` "Hidden" :`true` "Visible" :!type "ESlateVisibility Enum")))
    (:`else`)))

(event `self.ReceiveBeginPlay`
  ;[1 0 0] Begin Play
  (`parent.ReceiveBeginPlay`)
  (`/Game/CombatSystem/Blueprints/Components/BP_CollisionComponent.SetCollisionMeshComponent` (`self.MainWeaponCollisionComponent`) (`self.WeaponMesh`))
  (bind _returnvalue (`|CreateWidget` "/Game/CombatSystem/UI/WB_BossHealth.WB_BossHealth_C" (`GameplayStatics.GetPlayerController` 0)))
  (bind _output_get (set `self.BossHealthUI` _returnvalue))
  (`/Game/CombatSystem/UI/WB_BossHealth.Initialize` _output_get (`self.StatsComponent`))
  (`UserWidget.AddToViewport` (`self.BossHealthUI`) 0))

(event `self.OnTargetSet`
  (params (NewTarget :type "Actor Object Reference"))
  ;[1 1 1] Display Boss Health when enemy targets player
  (`parent.OnTargetSet` NewTarget)
  (`self.SetBossHealthVisibility` (`KismetSystemLibrary.IsValid` NewTarget)))

(event `self.MainWeaponCollisionComponent.OnHit`
  (params (HitResult :type "HitResult Structure"))
  (bind (_bblockinghit _binitialoverlap _time _distance _location _impactpoint _normal _impactnormal _physmat _hitactor) (`GameplayStatics.BreakHitResult` HitResult))
  ;[1 1 1] On Hit Event
  (bind _returnvalue (message `/Game/CombatSystem/Blueprints/Interfaces/Combat_BPI.CanReceiveDamage` _hitactor))
  (if _returnvalue
    (`GameplayStatics.ApplyPointDamage` _hitactor (`/Game/CombatSystem/Blueprints/Components/BP_StatsComponent.GetCurrentStatValue` (`self.StatsComponent`) "NewEnumerator4") (`self.GetActorForwardVector`) HitResult (`self.GetController`) self "/Game/CombatSystem/Blueprints/DamageTypes/BP_AttackDamageType.BP_AttackDamageType_C")))

(event `/Game/CombatSystem/Blueprints/Interfaces/Targeting_BPI.OnTargeted`
  (params (bIsTargeted :type Boolean))
  ;[1 1 1] Targeting Event
  (`parent.OnTargeted` bIsTargeted))

(event `SimulateWeaponPhysics`
  (bind _weaponmesh (`self.WeaponMesh`))
  ;[1 1 1] Simulate Physics
  (`PrimitiveComponent.SetCollisionProfileName` _weaponmesh "PhysicsActor" true)
  (`PrimitiveComponent.SetSimulatePhysics` _weaponmesh false))

(event `self.PerformDeath`
  ;[1 1 1] Perform Death
  (`parent.PerformDeath`)
  (`self.SimulateWeaponPhysics`)
  (`self.SetBossHealthVisibility` false))

(event `self.CombatComponent.OnCombatToggled`
  (params (bIsCombatEnabled :type Boolean))
  ;[1 1 1] Attach Weapon to sockets
  (`SceneComponent.K2_AttachToComponent` (`self.WeaponMesh`) (`self.Mesh`) (select `bool` bIsCombatEnabled :`false` (`self.AttachSocketName`) :`true` (`self.WeaponHandSocketName`)) "KeepRelative" "KeepRelative" "KeepRelative" true))

(fn `UserConstructionScript`
  (`parent.UserConstructionScript`))