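; BP_TestDummyCharacter is a test dummy character for the combat system that can be targeted by lock-on.
; On BeginPlay it initializes its StatsComponent, then spawns each StartingEquipment class with itself as owner and instigator and calls OnEquipped.
; OnTargeted toggles the LockOnWidget's visibility to match the targeted state.
; CanBeTargeted queries StateManagerComponent and refuses targeting while the dummy is in the Dead state.
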(event `self.ReceiveBeginPlay`
  ;[1 1 1] Begin Play
  (`/Game/CombatSystem/Blueprints/Components/BP_StatsComponent.InitializeStats` (`self.StatsComponent`))
  (for _array_element (`self.StartingEquipment`)
    (bind _returnvalue (`|SpawnActorFromClass` _array_element (`self.GetTransform`) "Undefined" "OverrideRootScale" self self))
    (`/Game/CombatSystem/Blueprints/Actors/BP_BaseEquipable.OnEquipped` _returnvalue)))

(event `/Game/CombatSystem/Blueprints/Interfaces/Targeting_BPI.OnTargeted`
  (params (bIsTargeted :type Boolean))
  (`SceneComponent.SetVisibility` (`self.Lock-OnWidget`) bIsTargeted false))

(fn `CanBeTargeted`
  (returns (ReturnValue :type Boolean))
  (return (not (`/Game/CombatSystem/Blueprints/Components/BP_StateManagerComponent.IsCurrentStateEqualToAny` (`self.StateManagerComponent`) (struct :`GameplayTags` (struct :`(TagName` "Character.State.Dead")))))))

(fn `UserConstructionScript`
  (`parent.UserConstructionScript`))