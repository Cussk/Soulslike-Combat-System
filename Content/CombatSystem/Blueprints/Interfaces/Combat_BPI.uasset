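; Combat_BPI is a Blueprint Interface that defines the shared contract for characters in the combat system.
; It covers attack and action execution with montage selection and durations, combo continuation and resets, and weapon collision toggling.
; It also exposes i-frames, damage eligibility, movement and rotation control, and health potion count updates.
; The file holds only signatures with default returns, leaving behaviour to implementers.
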(fn `ActivateCollision`
  (params (CollisionPart :type "/Game/CombatSystem/Blueprints/Enums/ECollisionPart Enum" :default "NewEnumerator0")))

(fn `CanReceiveDamage`
  (returns (ReturnValue :type Boolean))
  (return false))

(fn `ContinueAttack`)

(fn `DeactivateCollision`
  (params (CollisionPart :type "/Game/CombatSystem/Blueprints/Enums/ECollisionPart Enum" :default "NewEnumerator0")))

(fn `GetDesiredRotation`
  (returns (ReturnValue :type "Rotator Structure"))
  (return))

(fn `GetMovementSpeedMode`
  (returns (ReturnValue :type "/Game/CombatSystem/Blueprints/Enums/E_MovementSpeedMode Enum"))
  (return "NewEnumerator0"))

(fn `PerformAction`
  (params (ActionTag :type "GameplayTag Structure") (StateTag :type "GameplayTag Structure" :default (struct :`TagName` "Character.State.General Action State")) (MontageIndex :type Integer) (bRandomIndex :type Boolean))
  (returns (IsSuccess :type Boolean) (ActionDuration :type "Float (double-precision)"))
  (return false 0.0))

(fn `PerformAttack`
  (params (AttackType :type "GameplayTag Structure") (AttackIndex :type Integer) (bRandomIndex :type Boolean))
  (returns (IsSuccess :type Boolean) (AttackDuration :type "Float (double-precision)"))
  (return false 0.0))

(fn `PerformCustomAction`
  (params (ActionTag :type "GameplayTag Structure") (StateTag :type "GameplayTag Structure") (InMontgae :type "AnimMontage Object Reference") (MontagePlayRate :type "Float (double-precision)" :default 1.0) (bAutoReset :type Boolean))
  (returns (bIsSuccess :type Boolean))
  (return false))

(fn `ResetAttack`)

(fn `ResetCombat`)

(fn `RotateToTarget`)

(fn `SetCanMove`
  (params (bCanMove :type Boolean)))

(fn `SetIFrames`
  (params (bEnableIFrames :type Boolean)))

(fn `UpdateHealthPotionAmount`
  (params (Amount :type Integer)))